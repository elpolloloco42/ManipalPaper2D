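; BP_Claw is a 2D enemy claw that hides below its placed position and lunges upward when a Paper2DHero enters its detection box.
; A timeline lerps it from the lowered start to the placed spot, replaying until the hero leaves.
; DoOnce gates toggle flipbook visibility around the timeline's halfway value.
; It extends its parent's activation and randomly drops either rings or a health or mushroom pickup at the raised position.
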(event `self.ReceiveBeginPlay`
  ;[1 0.1235 0.1732] Begin play
  (`parent.ReceiveBeginPlay`)
  (`self.K2_SetActorLocation` (`self.start_location`))
  (`SceneComponent.SetVisibility` (`self.PaperFlipbook`) false false))

(event `Attack`
  (params (attack :type Boolean))
  (bind _paperflipbook (`self.PaperFlipbook`))
  ;[0.4078 1 0.3922] Attack Movement
  (bind (_direction _delta) (`Timeline|timeline_claw_movement` :!label _label)
    (:`Update`
      (`self.K2_SetActorLocation` (`KismetMathLibrary.VLerp` (`self.start_location`) (`self.end_location`) _delta))
      (`/Engine/EditorBlueprintResources/StandardMacros.CompareFloat` _delta 0.5
        (:`>`
          (`/Engine/EditorBlueprintResources/StandardMacros.DoOnce` false :!label _label_2
            (:`Completed`
              (`SceneComponent.SetVisibility` _paperflipbook true false)
              (goto _label_3 :!via `Reset`))))
        (:`<`
          (`/Engine/EditorBlueprintResources/StandardMacros.DoOnce` false :!label _label_3
            (:`Completed`
              (`SceneComponent.SetVisibility` _paperflipbook false false)
              (goto _label_2 :!via `Reset`))))))
    (:`Finished`
      (if attack
        (goto _label :!via `PlayFromStart`)
        (else
          (goto _label :!via `Stop`))))))

(event `self.DetectionBox.OnComponentBeginOverlap`
  (params (OverlappedComponent :type "PrimitiveComponent Object Reference") (OtherActor :type "Actor Object Reference") (OtherComp :type "PrimitiveComponent Object Reference") (OtherBodyIndex :type Integer) (bFromSweep :type Boolean) (SweepResult :type "HitResult Structure (by ref)"))
  ;[1 0.1216 0.1725] Overlap
  (cast `/Game/Blueprints/Hero/Paper2DHero` OtherActor)
  (`self.Attack` true))

(event `self.DetectionBox.OnComponentEndOverlap`
  (params (OverlappedComponent :type "PrimitiveComponent Object Reference") (OtherActor :type "Actor Object Reference") (OtherComp :type "PrimitiveComponent Object Reference") (OtherBodyIndex :type Integer))
  ;[1 0.1216 0.1725] Overlap
  (cast `/Game/Blueprints/Hero/Paper2DHero` OtherActor)
  (`self.Attack` false))

(event `self.ActivateEnemie`
  (params (Active :type Boolean))
  ;[1 0.1216 0.1725] Override Activate Function
  (`parent.ActivateEnemie` Active)
  (set `self.active` (not Active)))

(event `self.DropItem`
  (bind _returnvalue (`self.K2_GetActorRotation`))
  (bind _end_location (`self.end_location`))
  (`/Engine/EditorBlueprintResources/StandardMacros.CompareFloat` (`KismetMathLibrary.RandomFloatInRange` 0.0 100.0) (`self.special_item_pop`)
    (:`>`
      (for _ (range (+ (`KismetMathLibrary.RandomIntegerInRange` 0 (`self.max_ring_dropped`)) 1))
        (`|SpawnActorFromClass` "/Game/Blueprints/PickUp/BP_PickUp_Ring.BP_PickUp_Ring_C" (`KismetMathLibrary.MakeTransform` _end_location _returnvalue) "Undefined" "OverrideRootScale")))
    (:`<`
      (`|SpawnActorFromClass` (select `bool` (`KismetMathLibrary.RandomBool`) :`false` "/Game/Blueprints/PickUp/BP_PickUpMushroom.BP_PickUpMushroom_C" :`true` "/Game/Blueprints/PickUp/BP_PickUp_Health.BP_PickUp_Health_C" :!type "Actor Class Reference") (`KismetMathLibrary.MakeTransform` _end_location _returnvalue) "Undefined" "OverrideRootScale"))))

(fn `UserConstructionScript`
  (bind _returnvalue (`self.K2_GetActorLocation`))
  (`PaperFlipbookComponent.SetFlipbook` (`self.PaperFlipbook`) "/Game/Animations/Claw.Claw")
  (set `self.delta` 50.0)
  (`parent.UserConstructionScript`)
  (set `self.end_location` _returnvalue)
  (set `self.start_location` (`KismetMathLibrary.MakeVector` (.x _returnvalue) (.y _returnvalue) (- (.z _returnvalue) (* 3 (.z (`.BoxExtent` (`KismetSystemLibrary.GetComponentBounds` (`self.Box`)))))))))