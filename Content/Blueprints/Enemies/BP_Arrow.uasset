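; BP_Arrow is a trap-fired arrow that damages the Paper2D hero on hit and destroys itself.
; Hitting anything else plays a Wobble timeline that rotates the scene component to mimic an impact shudder and disables collision.
; After the wobble and a short delay, the arrow removes itself from the owning trap's ArrowList and is destroyed; the hero-hit path skips that list removal.
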(event `self.ReceiveHit`
  (params (MyComp :type "PrimitiveComponent Object Reference") (Other :type "Actor Object Reference") (OtherComp :type "PrimitiveComponent Object Reference") (bSelfMoved :type Boolean) (HitLocation :type "Vector Structure") (HitNormal :type "Vector Structure") (NormalImpulse :type "Vector Structure") (Hit :type "HitResult Structure (by ref)"))
  (bind _aspaper_2dhero (cast `/Game/Blueprints/Hero/Paper2DHero` Other)
    (:`then`
      (bind _output_get (set `self.paper_player_ref` _aspaper_2dhero))
      (`GameplayStatics.ApplyDamage` _output_get 1.0)
      (`self.K2_DestroyActor`))
    (:`CastFailed`
      (bind (_direction _wobble) (`Timeline|Wobble` :!via `PlayFromStart`)
        (:`Update`
          (`SceneComponent.K2_SetRelativeRotation` (`self.Scene`) (`KismetMathLibrary.RLerp` (struct) (struct :`Pitch` 100.0) _wobble) false false)
          (`PrimitiveComponent.SetCollisionEnabled` (`self.Collision`) "NoCollision"))
        (:`Finished`
          (`KismetSystemLibrary.Delay` 2.0)
          (`KismetArrayLibrary.Array_RemoveItem` (`/Game/Blueprints/Enemies/BP_ArrowTrap.arrow_list` (`self.trap_ref`)) self)
          (`self.K2_DestroyActor`))))))

(fn `UserConstructionScript`)