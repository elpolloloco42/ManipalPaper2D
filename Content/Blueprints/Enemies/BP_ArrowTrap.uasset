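; Arrow trap enemy that fires BP_Arrow projectiles on a looping timer while a timeline moves it along an offset from its start position.
; BeginPlay rotates the trap by its Orientation; the construction script derives the movement offset from Orientation, Speed and the spawn point's rotation.
; The ActivateEnemie override pauses or resumes both firing and movement, and shows or hides every arrow tracked in ArrowList.
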(event `self.ReceiveBeginPlay`
  ;[1 0.1216 0.1725] Event begin play
  (set `self.start_position` (`self.K2_GetActorLocation`))
  (bind _returnvalue (`KismetSystemLibrary.K2_SetTimer` null "Fire" 1.5 true))
  (set `self.arrow_timer` _returnvalue)
  (`SceneComponent.K2_AddRelativeRotation` (`self.Scene`) (select `/Game/Data/E_Orientation` (`self.orientation`) :`NewEnumerator0` (struct :`Pitch` 90.0) :`NewEnumerator1` (struct :`Pitch` 270.0) :`NewEnumerator3` (struct :`Pitch` 180.0) :!type "Rotator Structure") false false)
  (`self.ActivateEnemie` (`self.active`)))

(event `self.ActivateEnemie`
  (params (Active :type Boolean))
  (bind _arrow_timer (`self.arrow_timer`))
  (bind _start_position (`self.start_position`))
  ;[1 0.1216 0.1725] Override Activate Function
  (`parent.ActivateEnemie` Active)
  (for _array_element (`self.arrow_list`)
    (`SceneComponent.SetVisibility` (`/Game/Blueprints/Enemies/BP_Arrow.Scene` _array_element) Active true))
  (if Active
    (`KismetSystemLibrary.K2_UnPauseTimerHandle` _arrow_timer)
    (bind (_direction _movement) (`Timeline|Timeline_Trap_Movement` :!label _label)
      (:`Update`
        (`self.K2_SetActorLocation` (`KismetMathLibrary.VLerp` _start_position (+ _start_position (`self.movement_vector`)) _movement))))
    (else
      (`KismetSystemLibrary.K2_PauseTimerHandle` _arrow_timer)
      (goto _label :!via `Stop`))))

(event `Fire`
  (bind (_returnvalue_location _returnvalue_rotation _returnvalue_scale) (`KismetMathLibrary.BreakTransform` (`SceneComponent.K2_GetComponentToWorld` (`self.SpawnPoint`))))
  ;[0.4078 1 0.3922] Fire
  (if (`self.active`)
    (bind _returnvalue (`|SpawnActorFromClass` "/Game/Blueprints/Enemies/BP_Arrow.BP_Arrow_C" (`KismetMathLibrary.MakeTransform` (+ _returnvalue_location (0.0 -0.1 0.0)) _returnvalue_rotation _returnvalue_scale) "Undefined" "OverrideRootScale" null self))
    (`KismetArrayLibrary.Array_Add` (`self.arrow_list`) _returnvalue)))

(event `self.ReceiveTick`
  (params (DeltaSeconds :type "Float (single-precision)")))

(fn `UserConstructionScript`
  (bind _speed (`self.speed`))
  (bind _returnvalue (`KismetMathLibrary.MakeVector` 0.0 0.0 _speed))
  (bind _returnvalue_2 (`KismetMathLibrary.MakeVector` _speed))
  (bind (_returnvalue_location _returnvalue_rotation) (`KismetMathLibrary.BreakTransform` (`SceneComponent.K2_GetComponentToWorld` (`self.SpawnPoint`))))
  (set `self.movement_vector` (`KismetMathLibrary.TransformDirection` (`KismetMathLibrary.MakeTransform` (0.0 0.0 0.0) _returnvalue_rotation) (select `/Game/Data/E_Orientation` (`self.orientation`) :`NewEnumerator0` _returnvalue_2 :`NewEnumerator1` _returnvalue_2 :`NewEnumerator2` _returnvalue :`NewEnumerator3` _returnvalue))))