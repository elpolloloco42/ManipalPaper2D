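; Base enemy Blueprint for a Paper2D game that damages the player on contact through the player controller.
; Any damage kills it, dropping either a random number of rings or a health or mushroom pickup based on a chance roll, then removing it from the GameState.
; The construction script sizes the collision box from the flipbook bounds, and ActivateEnemie sets an active flag and toggles visibility.
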(event `self.ReceiveBeginPlay`
  ;[1 0.1412 0.2039] BeginPlay
  (bind _aspaper_2dgame_state_base (cast `/Game/Blueprints/Paper2DGameStateBase` (`GameplayStatics.GetGameState`)))
  (set `self.game_state_ref` _aspaper_2dgame_state_base))

(event `self.Box.OnComponentBeginOverlap`
  (params (OverlappedComponent :type "PrimitiveComponent Object Reference") (OtherActor :type "Actor Object Reference") (OtherComp :type "PrimitiveComponent Object Reference") (OtherBodyIndex :type Integer) (bFromSweep :type Boolean) (SweepResult :type "HitResult Structure (by ref)"))
  ;[1 0.1412 0.2039] Overlap player and damage him
  (cast `/Game/Blueprints/Hero/Paper2DHero` OtherActor)
  (bind _aspaper_2dcontroller (cast `/Game/Blueprints/Paper2DController` (`GameplayStatics.GetPlayerController` 0)))
  (`/Game/Blueprints/Paper2DController.OnDamage` _aspaper_2dcontroller))

(event `self.ReceiveAnyDamage`
  (params (Damage :type "Float (single-precision)") (DamageType :type "DamageType Object Reference") (InstigatedBy :type "Controller Object Reference") (DamageCauser :type "Actor Object Reference"))
  ;[1 0.6471 0.2902] Death and drop random item function
  (`PrimitiveComponent.SetCollisionEnabled` (`self.Box`) "NoCollision")
  (`self.DropItem`)
  (`/Game/Blueprints/Paper2DGameStateBase.RemoveEnemies` (`self.game_state_ref`) self)
  (`self.K2_DestroyActor`))

(event `DropItem`
  (bind (_returnvalue_location _returnvalue_rotation) (`KismetMathLibrary.BreakTransform` (`self.GetTransform`)))
  ;[1 0.6471 0.2902] Death and drop random item function
  (`/Engine/EditorBlueprintResources/StandardMacros.CompareFloat` (`KismetMathLibrary.RandomFloatInRange` 0.0 100.0) (`self.special_item_pop`)
    (:`>`
      (for _ (range (+ (`KismetMathLibrary.RandomIntegerInRange` 0 (`self.max_ring_dropped`)) 1))
        (`|SpawnActorFromClass` "/Game/Blueprints/PickUp/BP_PickUp_Ring.BP_PickUp_Ring_C" (`KismetMathLibrary.MakeTransform` _returnvalue_location _returnvalue_rotation) "Undefined" "OverrideRootScale")))
    (:`<`
      (`|SpawnActorFromClass` (select `bool` (`KismetMathLibrary.RandomBool`) :`false` "/Game/Blueprints/PickUp/BP_PickUpMushroom.BP_PickUpMushroom_C" :`true` "/Game/Blueprints/PickUp/BP_PickUp_Health.BP_PickUp_Health_C" :!type "Actor Class Reference") (`KismetMathLibrary.MakeTransform` _returnvalue_location _returnvalue_rotation) "Undefined" "OverrideRootScale"))))

(fn `ActivateEnemie`
  (params (Active :type Boolean))
  (bind _output_get (set `self.active` Active))
  (`self.SetActorHiddenInGame` (not _output_get)))

(fn `UserConstructionScript`
  (bind (_returnvalue_x _returnvalue_y _returnvalue_z) (`KismetMathLibrary.BreakVector` (`KismetMathLibrary.TransformDirection` (`KismetMathLibrary.MakeTransform` (0.0 0.0 0.0) (`self.K2_GetActorRotation`)) (`.BoxExtent` (`KismetSystemLibrary.GetComponentBounds` (`self.PaperFlipbook`))))))
  ;[0.3325 0.162 0.3864] Set collision scale to sprite scale
  (`BoxComponent.SetBoxExtent` (`self.Box`) (`KismetMathLibrary.MakeVector` (`KismetMathLibrary.Abs` _returnvalue_x) 50.0 (+ (`KismetMathLibrary.Abs` _returnvalue_z) (`self.delta`))) true))