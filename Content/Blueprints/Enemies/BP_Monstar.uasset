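; BP_Monstar is an enemy Blueprint that patrols between two points using a walking flipbook sprite.
; Its ActivateEnemie override starts or stops a timeline that lerps the actor from StartLocation to EndLocation and restarts on finish while active.
; The sprite is mirrored through its X scale when the timeline value nears either end.
; The construction script sets the flipbook and captures StartLocation from the actor's placed position.
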(event `self.ActivateEnemie`
  (params (Active :type Boolean))
  (bind _paperflipbook (`self.PaperFlipbook`))
  ;[1 0.1216 0.1725] Override Activate Function
  (`parent.ActivateEnemie` Active)
  (if Active
    (bind (_direction _delta) (`Timeline|timeline_monstar_movement` :`NewTime` 2.0 :!label _label)
      (:`Update`
        (`self.K2_SetActorLocation` (`KismetMathLibrary.VLerp` (`self.start_location`) (`self.end_location`) _delta))
        (if (<= _delta 0.01)
          (`SceneComponent.SetWorldScale3D` _paperflipbook (-1.0 1.0 1.0))
          (elif (>= _delta 0.99)
            (`SceneComponent.SetWorldScale3D` _paperflipbook (1.0 1.0 1.0)))))
      (:`Finished`
        (if (`self.active`)
          (goto _label :!via `PlayFromStart`))))
    (else
      (goto _label :!via `Stop`))))

(fn `UserConstructionScript`
  (`PaperFlipbookComponent.SetFlipbook` (`self.PaperFlipbook`) "/Game/Animations/monstar_walk.monstar_walk")
  (set `self.start_location` (`self.K2_GetActorLocation`))
  (set `self.delta` 0.0)
  (`parent.UserConstructionScript`))