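; BP_Projectile is a hero projectile with a Paper2D sprite that damages enemies derived from BP_IA_Enemie_Base.
; On any hit it applies damage if the other actor is such an enemy, then hides the sprite and ignores the Vehicle collision channel.
; It swaps its particle system to an explosion and destroys itself after a short delay.
; A timer from BeginPlay also destroys it after a few seconds.
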(event `self.ReceiveHit`
  (params (MyComp :type "PrimitiveComponent Object Reference") (Other :type "Actor Object Reference") (OtherComp :type "PrimitiveComponent Object Reference") (bSelfMoved :type Boolean) (HitLocation :type "Vector Structure") (HitNormal :type "Vector Structure") (NormalImpulse :type "Vector Structure") (Hit :type "HitResult Structure (by ref)"))
  (bind _papersprite (`self.PaperSprite`))
  (`|ExecutionSequence`
    (:`then_0`
      (bind _asbp_ia_enemie_base (cast `/Game/Blueprints/Enemies/BP_IA_Enemie_Base` Other))
      (`GameplayStatics.ApplyDamage` _asbp_ia_enemie_base 1.0))
    (:`then_1`
      (`SceneComponent.SetVisibility` _papersprite false false)
      (`PrimitiveComponent.SetCollisionResponseToChannel` _papersprite "ECC_Vehicle" "ECR_Ignore")
      (`ParticleSystemComponent.SetTemplate` (`self.ParticleSystem`) "/Game/StarterContent/Particles/P_Explosion.P_Explosion")
      (`KismetSystemLibrary.Delay` 1.0)
      (`self.K2_DestroyActor`))))

(event `self.ReceiveBeginPlay`
  (`KismetSystemLibrary.Delay` 5.0)
  (`self.K2_DestroyActor`))

(fn `UserConstructionScript`
  (`self.SetActorScale3D` (1.0 1.0 1.0)))