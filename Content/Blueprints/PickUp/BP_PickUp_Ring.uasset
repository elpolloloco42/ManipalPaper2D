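; Ring pickup that pops out with a random physics launch when it begins play.
; BeginPlay builds a Force-scaled velocity within a Direction-degree spread around up in the actor's local XZ plane, rotates it by actor rotation and applies it to Sphere.
; Sphere is locked to YZ when the rotated X is near zero, otherwise XZ.
; GetBlockConstraint holds a similar plane test with inverted bounds, unused here.
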(event `self.ReceiveBeginPlay`
  (bind _sphere (`self.Sphere`))
  (bind _direction (`self.direction`))
  (bind _force (`self.force`))
  (bind _returnvalue (`KismetMathLibrary.RandomFloatInRange` (* _direction -1.0) _direction))
  (bind _returnvalue_2 (`KismetMathLibrary.GreaterGreater_VectorRotator` (`KismetMathLibrary.MakeVector` (* (`KismetMathLibrary.DegSin` _returnvalue) _force) 0.0 (* _force (`KismetMathLibrary.DegCos` _returnvalue))) (`self.K2_GetActorRotation`)))
  ;[1 0.1412 0.2039] Begin Play
  (`parent.ReceiveBeginPlay`)
  (`PrimitiveComponent.SetConstraintMode` _sphere (select `bool` (`KismetMathLibrary.InRange_FloatFloat` (.x _returnvalue_2) -0.1 0.1) :`false` "XZPlane" :`true` "YZPlane" :!type "EDOFMode Enum"))
  (`PrimitiveComponent.SetAllPhysicsLinearVelocity` _sphere _returnvalue_2 false))

(fn `GetBlockConstraint`
  (params (vector :type "Vector Structure"))
  (returns (EDOFMode :type "EDOFMode Enum"))
  (if (`KismetMathLibrary.InRange_FloatFloat` vector_X 0.1 -0.1)
    (return "YZPlane")
    (else
      (return "XZPlane"))))

(fn `UserConstructionScript`
  (`parent.UserConstructionScript`))