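; Game state for a Paper2D platformer that builds rooms from tile maps and tracks worlds and the current room.
; BeginPlay scans each BP_Room's tile user data to spawn merged platforms, paired-marker Monstars, Claws and doors, then chains doors cyclically.
; ChangeWorld toggles tilemaps, doors and enemies by world, initially hiding all but the first.
; Camera functions derive room bounds and return clamped edge positions, unrotating vectors to support rotated tile maps.
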(event `self.ReceiveBeginPlay`
  ;[1 0.1412 0.2039] Begin Play
  (`|ExecutionSequence`
    (:`then_0`
      (`KismetSystemLibrary.PrintString` "[GAME STATE]"))
    (:`then_1`
      (bind _aspaper_2dcontroller (cast `/Game/Blueprints/Paper2DController` (`GameplayStatics.GetPlayerController` 0)))
      (set `self.player_controller_ref` _aspaper_2dcontroller))
    (:`then_2`
      (bind _outactors (`GameplayStatics.GetAllActorsOfClass` "/Game/Blueprints/Level/BP_Room.BP_Room_C"))
      (for _array_element _outactors
        (bind _struct_room (`self.MakeStructRoom` _array_element))
        (`KismetArrayLibrary.Array_Add` (`self.room_list`) _struct_room)
        (`KismetArrayLibrary.Array_AddUnique` (`self.world_id_list`) (`/Game/Blueprints/Level/BP_Room.world_id` _array_element)))
      (for _array_element_2 (`self.world_id_list`)
        (if (!= _array_element_2 (`self.first_world_id`))
          (`self.ChangeWorld` _array_element_2))))
    (:`then_3`
      (`self.InitDoorsConnexions`)
      (`self.UpdateCurrentRoomInfos` (`self.first_world_id`) (`self.first_room_id`))
      (`self.ComputeCameraLimit`))))

(event `InitDoorsConnexions`
  ;[1 0.1412 0.2039] Doors initialisation / Set next door reference
  (bind _outactors (`GameplayStatics.GetAllActorsOfClass` "/Game/Blueprints/Level/BP_Door.BP_Door_C"))
  (for (_array_element _array_index) _outactors
    (bind _returnvalue (+ _array_index 1))
    (set `/Game/Blueprints/Level/BP_Door.next_door_ref` (`KismetArrayLibrary.Array_Get` _outactors (select `bool` (== _returnvalue (`KismetArrayLibrary.Array_Length` _outactors)) :`false` _returnvalue)) _array_element)))

(fn `CameraStateMachine`
  (returns (cameraPosition :type "Vector Structure") (center :type Boolean))
  (locals (location_camera_state :type "/Game/Data/CameraLimiteState Enum"))
  (bind _limit_right (`self.limit_right`))
  (bind _limit_left (`self.limit_left`))
  (bind _paper_tile_map (break `/Game/Data/S_Room` (`self.current_room`)))
  (bind _returnvalue (`SceneComponent.K2_GetComponentRotation` _paper_tile_map))
  (bind (_returnvalue_x _returnvalue_y _returnvalue_z) (`KismetMathLibrary.BreakVector` (`KismetMathLibrary.LessLess_VectorRotator` (`SceneComponent.K2_GetComponentLocation` (`/Game/Blueprints/Paper2DController.hero_camera_ref` (`self.player_controller_ref`))) _returnvalue)))
  (bind (_returnvalue_x_2 _returnvalue_y_2 _returnvalue_z_2) (`KismetMathLibrary.BreakVector` (`KismetMathLibrary.LessLess_VectorRotator` (`SceneComponent.K2_GetComponentLocation` _paper_tile_map) _returnvalue)))
  (bind _returnvalue_2 (- _returnvalue_z_2 (`self.camera_down_limit`)))
  (bind _returnvalue_3 (- _returnvalue_z_2 (`self.camera_up_limit`)))
  (bind _returnvalue_4 (+ _returnvalue_x_2 (`self.camera_left_limit`)))
  (bind _returnvalue_5 (+ _returnvalue_x_2 (`self.camera_right_limit`)))
  (if (`self.limit_up`)
    (if _limit_right
      (set `local.location_camera_state` "NewEnumerator5")
      (elif _limit_left
        (set `local.location_camera_state` "NewEnumerator6")
        (else
          (set `local.location_camera_state` "NewEnumerator0"))))
    (elif (`self.limit_down`)
      (if _limit_right
        (set `local.location_camera_state` "NewEnumerator7")
        (elif _limit_left
          (set `local.location_camera_state` "NewEnumerator8")
          (else
            (set `local.location_camera_state` "NewEnumerator1"))))
      (elif _limit_right
        (set `local.location_camera_state` "NewEnumerator3")
        (elif _limit_left
          (set `local.location_camera_state` "NewEnumerator2")
          (else
            (set `local.location_camera_state` "NewEnumerator4")
            (return (0.0 0.0 0.0) true))))))
  (return (`KismetMathLibrary.GreaterGreater_VectorRotator` (select `/Game/Data/CameraLimiteState` (`local.location_camera_state`) :`NewEnumerator0` (`KismetMathLibrary.MakeVector` _returnvalue_x _returnvalue_y _returnvalue_3) :`NewEnumerator1` (`KismetMathLibrary.MakeVector` _returnvalue_x _returnvalue_y _returnvalue_2) :`NewEnumerator3` (`KismetMathLibrary.MakeVector` _returnvalue_5 _returnvalue_y _returnvalue_z) :`NewEnumerator2` (`KismetMathLibrary.MakeVector` _returnvalue_4 _returnvalue_y _returnvalue_z) :`NewEnumerator5` (`KismetMathLibrary.MakeVector` _returnvalue_5 _returnvalue_y _returnvalue_3) :`NewEnumerator6` (`KismetMathLibrary.MakeVector` _returnvalue_4 _returnvalue_y _returnvalue_3) :`NewEnumerator7` (`KismetMathLibrary.MakeVector` _returnvalue_5 _returnvalue_y _returnvalue_2) :`NewEnumerator8` (`KismetMathLibrary.MakeVector` _returnvalue_4 _returnvalue_y _returnvalue_2)) _returnvalue) false))

(fn `ChangeWorld`
  (params (world_id :type Integer) (visible :type Boolean))
  (locals (counter :type Boolean))
  (for _array_element (`self.room_list`)
    (bind (_paper_tile_map _world_id _room_id _room_width _room_height _tile_length _door_list _enemie_list) (break `/Game/Data/S_Room` _array_element))
    (if (== _world_id world_id)
      (`SceneComponent.SetVisibility` _paper_tile_map visible false)
      (for _array_element_2 _door_list
        (`SceneComponent.SetVisibility` (`/Game/Blueprints/Level/BP_Door.Sprite` _array_element_2) visible false))
      (for _array_element_3 _enemie_list
        (`/Game/Blueprints/Enemies/BP_IA_Enemie_Base.ActivateEnemie` _array_element_3 visible)))))

(fn `CheckCameraLimit`
  (bind _player_controller_ref (`self.player_controller_ref`))
  (bind _paper_tile_map (break `/Game/Data/S_Room` (`self.current_room`)))
  (bind _returnvalue (`SceneComponent.K2_GetComponentLocation` (`/Game/Blueprints/Paper2DController.hero_camera_ref` _player_controller_ref)))
  (bind _returnvalue_2 (`SceneComponent.K2_GetComponentRotation` _paper_tile_map))
  (bind _returnvalue_3 (`SceneComponent.K2_GetComponentLocation` _paper_tile_map))
  (bind _returnvalue_x (`KismetMathLibrary.BreakVector` (`KismetMathLibrary.LessLess_VectorRotator` _returnvalue_3 _returnvalue_2)))
  (bind _returnvalue_x_2 (`KismetMathLibrary.BreakVector` (`KismetMathLibrary.LessLess_VectorRotator` _returnvalue _returnvalue_2)))
  (bind _z (.z _returnvalue))
  (bind _z_2 (.z _returnvalue_3))
  (bind _returnvalue_4 (- _returnvalue_x_2 _returnvalue_x))
  (`/Engine/EditorBlueprintResources/StandardMacros.IsValid` _player_controller_ref
    (:`Is Valid`
      (`|ExecutionSequence`
        (:`then_0`
          (if (>= _z (- _z_2 (`self.camera_up_limit`)))
            (set `self.limit_up` true)
            (set `self.limit_down` false)
            (else
              (set `self.limit_up` false)
              (if (<= _z (- _z_2 (`self.camera_down_limit`)))
                (set `self.limit_down` true)
                (else
                  (set `self.limit_down` false))))))
        (:`then_1`
          (if (>= _returnvalue_4 (`self.camera_right_limit`))
            (set `self.limit_right` true)
            (set `self.limit_left` false)
            (else
              (set `self.limit_right` false)
              (if (<= _returnvalue_4 (`self.camera_left_limit`))
                (set `self.limit_left` true)
                (else
                  (set `self.limit_left` false))))))))))

(fn `ComputeCameraLimit`
  (locals (map_width :type "Float (double-precision)") (map_height :type "Float (double-precision)") (delta :type "Float (double-precision)") (inverse_ratio :type "Float (double-precision)") (spring_length :type "Float (double-precision)"))
  (bind _player_controller_ref (`self.player_controller_ref`))
  (bind (_paper_tile_map _world_id _room_id _room_width _room_height _tile_length) (break `/Game/Data/S_Room` (`self.current_room`)))
  (`|ExecutionSequence`
    (:`then_0`
      (set `local.map_width` (* (`KismetMathLibrary.Conv_IntToDouble` _room_width) (`KismetMathLibrary.Conv_IntToDouble` _tile_length)))
      (set `local.map_height` (* (`KismetMathLibrary.Conv_IntToDouble` _room_height) (`KismetMathLibrary.Conv_IntToDouble` _tile_length)))
      (set `local.delta` (`KismetMathLibrary.Conv_IntToDouble` (/ _tile_length 2)))
      (set `local.inverse_ratio` (/ 1.0 (`CameraComponent.AspectRatio` (`/Game/Blueprints/Paper2DController.hero_camera_ref` _player_controller_ref))))
      (set `local.spring_length` (`KismetMathLibrary.Abs` (`SpringArmComponent.TargetArmLength` (`/Game/Blueprints/Hero/Paper2DHero.SpringArm` (`/Game/Blueprints/Paper2DController.player_ref` _player_controller_ref))))))
    (:`then_1`
      (set `self.camera_right_limit` (- (- (`local.map_width`) (`local.spring_length`)) (`local.delta`)))
      (set `self.camera_left_limit` (- (`local.spring_length`) (`local.delta`)))
      (set `self.camera_down_limit` (- (- (`local.map_height`) (`local.delta`)) (* (`local.inverse_ratio`) (`local.spring_length`))))
      (set `self.camera_up_limit` (- (* (`local.inverse_ratio`) (`local.spring_length`)) (`local.delta`))))))

(fn `GetTileWorldLocation`
  (params (P_counter :type "Float (double-precision)") (paper_tile_map :type "PaperTileMapComponent Object Reference") (column_index :type Integer) (line_index :type Integer) (tile_length :type Integer) (sprite_Y_offset :type "Float (double-precision)") (sprite_Z_offset :type "Float (double-precision)"))
  (returns (wolrd_location :type "Vector Structure") (world_rotation :type "Rotator Structure"))
  (locals (plateform_offset :type "Float (double-precision)"))
  (bind _returnvalue (`SceneComponent.K2_GetComponentRotation` paper_tile_map))
  (bind _returnvalue_2 (`KismetMathLibrary.Conv_IntToDouble` column_index))
  (bind (_returnvalue_x _returnvalue_y _returnvalue_z) (`KismetMathLibrary.BreakVector` (`KismetMathLibrary.LessLess_VectorRotator` (`SceneComponent.K2_GetComponentLocation` paper_tile_map) _returnvalue)))
  (bind (_returnvalue_x_2 _returnvalue_y_2 _returnvalue_z_2) (`KismetMathLibrary.BreakVector` (`KismetMathLibrary.GreaterGreater_VectorRotator` (`KismetMathLibrary.MakeVector` (+ _returnvalue_x (* (`local.plateform_offset`) (`KismetMathLibrary.Conv_IntToDouble` tile_length))) (- _returnvalue_y sprite_Z_offset) (- _returnvalue_z (`KismetMathLibrary.Conv_IntToDouble` (* line_index tile_length)))) _returnvalue)))
  (`|ExecutionSequence`
    (:`then_0`
      ;[0.09412 1 0.8706] Compute plateform offset
      (set `local.plateform_offset` (select `bool` (> P_counter 0.0) :`false` _returnvalue_2 :`true` (- _returnvalue_2 (+ (/ P_counter 2.0) 0.5)))))
    (:`then_1`
      ;[0.09412 1 0.8706] Compute world location
      (return (`KismetMathLibrary.MakeVector` _returnvalue_x_2 _returnvalue_y_2 (+ _returnvalue_z_2 sprite_Y_offset)) _returnvalue))))

(fn `MakeStructRoom`
  (params (class_room :type "/Game/Blueprints/Level/BP_Room Object Reference"))
  (returns (struct_room :type "/Game/Data/S_Room Structure"))
  (bind (_enmies_list _door_list) (`self.SpawnActorFromVisibleLayout` class_room))
  (return (make `/Game/Data/S_Room` (`/Game/Blueprints/Level/BP_Room.PaperTileMap` class_room) (`/Game/Blueprints/Level/BP_Room.world_id` class_room) (`/Game/Blueprints/Level/BP_Room.room_id` class_room) (`/Game/Blueprints/Level/BP_Room.map_width` class_room) (`/Game/Blueprints/Level/BP_Room.map_height` class_room) (`/Game/Blueprints/Level/BP_Room.tile_length` class_room) _door_list _enmies_list (`|MakeArray` null :!type "/Game/Blueprints/PickUp/BP_PickUpBase Object Reference"))))

(fn `RemoveEnemies`
  (params (Enemie :type "/Game/Blueprints/Enemies/BP_IA_Enemie_Base Object Reference"))
  (locals (save_index :type Integer))
  (bind _room_list (`self.room_list`))
  (bind _current_room (`self.current_room`))
  (set `local.save_index` (`KismetArrayLibrary.Array_Find` _room_list _current_room))
  (`KismetArrayLibrary.Array_RemoveItem` (`.enemie_list_21_7393B3D645A11015C06A269D64967A51` (break `/Game/Data/S_Room` (`self.current_room`))) Enemie)
  (`KismetArrayLibrary.Array_Set` _room_list (`local.save_index`) _current_room))

(fn `SpawnActorFromVisibleLayout`
  (params (room :type "/Game/Blueprints/Level/BP_Room Object Reference"))
  (returns (enmies_list :type "Array of /Game/Blueprints/Enemies/BP_IA_Enemie_Base Object Reference") (door_list :type "Array of /Game/Blueprints/Level/BP_Door Object Reference"))
  (locals (column_index :type Integer) (line_index :type Integer) (plateform_found :type Boolean) (size_counter :type "Float (double-precision)") (enemies_list :type "Array of /Game/Blueprints/Enemies/BP_IA_Enemie_Base Object Reference") (monstar_found :type Boolean) (end_monstar_location :type "Vector Structure") (room_tlp :type "/Game/Blueprints/Level/BP_Room Object Reference") (door_list_tmp :type "Array of /Game/Blueprints/Level/BP_Door Object Reference") (door_height :type "Float (double-precision)" :default 103.0))
  (bind _room_tlp (`local.room_tlp`))
  (bind _room_tlp_2 (`local.room_tlp`))
  (bind _room_tlp_3 (`local.room_tlp`))
  (bind _room_tlp_4 (`local.room_tlp`))
  (bind _room_tlp_5 (`local.room_tlp`))
  (bind _papertilemap (`/Game/Blueprints/Level/BP_Room.PaperTileMap` (`local.room_tlp`)))
  (bind _papertilemap_2 (`/Game/Blueprints/Level/BP_Room.PaperTileMap` (`local.room_tlp`)))
  (bind _papertilemap_3 (`/Game/Blueprints/Level/BP_Room.PaperTileMap` (`local.room_tlp`)))
  (bind _world_id (`/Game/Blueprints/Level/BP_Room.world_id` (`local.room_tlp`)))
  (bind _tile_length (`/Game/Blueprints/Level/BP_Room.tile_length` _room_tlp))
  (set `local.room_tlp` room)
  (for _index (range (+ (`/Game/Blueprints/Level/BP_Room.map_height` room) 1))
    (set `local.line_index` _index)
    (for _index_2 (range (+ (`/Game/Blueprints/Level/BP_Room.map_width` _room_tlp_3) 1))
      (set `local.column_index` _index_2)
      (switch `name` (`TileMapBlueprintLibrary.GetTileUserData` (`PaperTileMapComponent.GetTile` (`/Game/Blueprints/Level/BP_Room.PaperTileMap` _room_tlp_3) (`local.column_index`) (`local.line_index`) 1))
        (:`Default`
          ;[1 0.6471 0.2902] PLATEFORM: Compute plateform size / Set world location / Spawn actor
          (if (`local.plateform_found`)
            (set `local.plateform_found` false)
            (bind (_wolrd_location _world_rotation) (`self.GetTileWorldLocation` (`local.size_counter`) (`/Game/Blueprints/Level/BP_Room.PaperTileMap` _room_tlp_4) (`local.column_index`) (`local.line_index`) (`/Game/Blueprints/Level/BP_Room.tile_length` _room_tlp_4)))
            (`|SpawnActorFromClass` "/Game/Blueprints/Level/BP_Plateform.BP_Plateform_C" (`KismetMathLibrary.MakeTransform` _wolrd_location _world_rotation (`KismetMathLibrary.MakeVector` (`local.size_counter`) 1.0 1.0)) "Undefined" "OverrideRootScale")
            (set `local.size_counter` 0.0)))
        (:`monstar`
          ;[0.09412 1 0.8706] MONSTAR: Set the end point / Spawn actor
          (`PaperTileMapComponent.MakeTileMapEditable` _papertilemap_2)
          (`PaperTileMapComponent.SetTile` _papertilemap_2 (`local.column_index`) (`local.line_index`) 1 (`PaperTileMapComponent.GetTile` _papertilemap_2 0 0 0))
          (bind (_wolrd_location_2 _world_rotation_2) (`self.GetTileWorldLocation` 0.0 (`/Game/Blueprints/Level/BP_Room.PaperTileMap` _room_tlp_5) (`local.column_index`) (`local.line_index`) (`/Game/Blueprints/Level/BP_Room.tile_length` _room_tlp_5) -13.0 0.1))
          (if (`local.monstar_found`)
            (set `local.monstar_found` false)
            (bind _returnvalue (`|SpawnActorFromClass` "/Game/Blueprints/Enemies/BP_Monstar.BP_Monstar_C" (`KismetMathLibrary.MakeTransform` _wolrd_location_2 _world_rotation_2 (1.0 1.0 1.0)) "Undefined" "OverrideRootScale" null (`local.end_monstar_location`)))
            (`KismetArrayLibrary.Array_Add` (`local.enemies_list`) _returnvalue)
            (else
              (set `local.monstar_found` true)
              (set `local.end_monstar_location` _wolrd_location_2))))
        (:`claw`
          ;[0.09412 1 0.8706] CLAW
          (`PaperTileMapComponent.MakeTileMapEditable` _papertilemap)
          (`PaperTileMapComponent.SetTile` _papertilemap (`local.column_index`) (`local.line_index`) 1 (`PaperTileMapComponent.GetTile` _papertilemap 0 0 0))
          (bind (_wolrd_location_3 _world_rotation_3) (`self.GetTileWorldLocation` 0.0 (`/Game/Blueprints/Level/BP_Room.PaperTileMap` _room_tlp_2) (`local.column_index`) (`local.line_index`) (`/Game/Blueprints/Level/BP_Room.tile_length` _room_tlp_2) 50.0 0.1))
          (bind _returnvalue_2 (`|SpawnActorFromClass` "/Game/Blueprints/Enemies/BP_Claw.BP_Claw_C" (`KismetMathLibrary.MakeTransform` _wolrd_location_3 _world_rotation_3 (1.0 1.0 1.0)) "Undefined" "OverrideRootScale"))
          (`KismetArrayLibrary.Array_Add` (`local.enemies_list`) _returnvalue_2))
        (:`plateform`
          (`/Engine/EditorBlueprintResources/StandardMacros.IncrementFloat` (`local.size_counter`)
            (:`  `
              (if (not (`local.plateform_found`))
                (set `local.plateform_found` true)))))
        (:`door`
          ;[1 1 1] DOOR
          (`|ExecutionSequence`
            (:`then_0`
              (`PaperTileMapComponent.MakeTileMapEditable` _papertilemap_3)
              (`PaperTileMapComponent.SetTile` _papertilemap_3 (`local.column_index`) (`local.line_index`) 1 (`PaperTileMapComponent.GetTile` _papertilemap_3 0 0 0)))
            (:`then_1`
              (bind (_wolrd_location_4 _world_rotation_4) (`self.GetTileWorldLocation` 0.0 (`/Game/Blueprints/Level/BP_Room.PaperTileMap` _room_tlp) (`local.column_index`) (`local.line_index`) _tile_length (- (`local.door_height`) (`KismetMathLibrary.Conv_IntToDouble` (/ _tile_length 2))) 0.1))
              (bind _returnvalue_3 (`|SpawnActorFromClass` "/Game/Blueprints/Level/BP_Door.BP_Door_C" (`KismetMathLibrary.MakeTransform` _wolrd_location_4 _world_rotation_4 (1.0 1.0 1.0)) "Undefined" "OverrideRootScale" null (select `int` _world_id :`0` "/Game/Sprites/Objects/door_2.door_2" :`1` "/Game/Sprites/Objects/door_3.door_3" :`2` "/Game/Sprites/Objects/door_1.door_1" :!type "PaperSprite Object Reference") _world_id))
              (`KismetArrayLibrary.Array_Add` (`local.door_list_tmp`) _returnvalue_3)))))))
  (return (`local.enemies_list`) (`local.door_list_tmp`)))

(fn `UpdateCurrentRoomInfos`
  (params (world_id :type Integer) (room_id :type Integer))
  (if (== world_id (`self.first_world_id`))
    (for _array_element (`self.room_list`)
      (if (== (`.room_id_9_1C4B5A78497AAF2225184C9F6C54E3DC` (break `/Game/Data/S_Room` _array_element)) room_id)
        (set `self.current_room` _array_element)
        (break)))))

(fn `UserConstructionScript`)