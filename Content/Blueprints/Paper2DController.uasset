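; Player controller for a 2D Paper hero, turning input into movement, multi-jumps, wall jumps, dashes and ladder climbing.
; Line traces pick wall jump or rejump and find drop-through platforms, while counters cap jumps and dashes.
; Doors switch worlds and rooms, re-orient sprite and spring arm, and blend spawned cameras, though Tick resets view to hero as state-machine logic is unwired.
; It also tracks health, damage and pickups, updating the HUD.
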(event `InputAxis|Move_horizontal`
  (params (AxisValue :type "Float (single-precision)"))
  (bind _player_ref (`self.player_ref`))
  ;[0.09412 1 0.8706] Movement control
  (if (`self.can_move_horizontaly`)
    (`Pawn.AddMovementInput` _player_ref (`SceneComponent.GetForwardVector` (`PaperCharacter.Sprite` _player_ref)) AxisValue false)))

(event `InputAction|Jump`
  (params (Key :type "Key Structure" :default "AnyKey"))
  (bind _player_ref (`self.player_ref`))
  ;[0.07248 0.645 0.1291] Jump / Wall Jump
  (:`Pressed`
    (set `self.can_move_horizontaly` true)
    (set `self.can_climb` false)
    (`|ExecutionSequence`
      (:`then_0`
        (if (`Character.CanJump` _player_ref)
          (`Character.Jump` _player_ref)
          (else
            (`self.MultiJump`))))
      (:`then_1`
        (set `/Game/Blueprints/Hero/Paper2DHero.is_damaged` false (`self.player_ref`)))))
  (:`Released`
    (`Character.StopJumping` (`self.player_ref`))))

(event `Key|D`
  (params (Key :type "Key Structure" :default "AnyKey"))
  ;[0.09412 1 0.8706] Movement control
  (:`Pressed`
    (`SceneComponent.K2_SetRelativeRotation` (`self.hero_flipbook_ref`) (struct) false false)))

(event `Key|Q`
  (params (Key :type "Key Structure" :default "AnyKey"))
  ;[0.09412 1 0.8706] Movement control
  (:`Pressed`
    (`SceneComponent.K2_SetRelativeRotation` (`self.hero_flipbook_ref`) (struct :`Yaw` 180.0) false false)))

(event `InputAxis|Move_vertical`
  (params (AxisValue :type "Float (single-precision)"))
  (bind _player_ref (`self.player_ref`))
  ;[1 1 1] UNUSE
  ;;[1 1 1] Ladder functions
  (if (`self.can_climb`)
    (if (not (`KismetMathLibrary.InRange_FloatFloat` AxisValue -0.1 0.1))
      (set `/Game/Blueprints/Hero/Paper2DHero.is_climbing` true (`self.player_ref`))
      (set `self.can_move_horizontaly` false)
      (`PaperFlipbookComponent.SetPlayRate` (`self.hero_flipbook_ref`) 1.0)
      (`CharacterMovementComponent.SetMovementMode` (`Character.CharacterMovement` _player_ref) "MOVE_Flying" 0)
      (`Pawn.AddMovementInput` _player_ref (0.0 0.0 0.5) AxisValue false))))

(event `self.ReceiveBeginPlay`
  (bind _player_ref (`self.player_ref`))
  ;[1 0.1412 0.2039] Begin play / Reset Counter on landing
  (`|ExecutionSequence`
    (:`then_0`
      (`KismetSystemLibrary.PrintString` "[PAPER2DCONTROLLER]"))
    (:`then_1`
      (bind _counter (`/Engine/EditorBlueprintResources/StandardMacros.Do N` 2 :!label _label)
        (:`Exit`
          (bind _returnvalue (`|SpawnActorFromClass` "/Script/Engine.CameraActor" (`KismetMathLibrary.MakeTransform` (0.0 0.0 0.0)) "Undefined" "OverrideRootScale"))
          (switch `int` _counter
            (:`1`
              (set `self.pursuit_camera_ref` _returnvalue))
            (:`2`
              (set `self.transition_camera_ref` _returnvalue)))
          (`CameraComponent.SetConstraintAspectRatio` (`CameraActor.CameraComponent` (select `int` _counter :`0` null :`1` (`self.pursuit_camera_ref`) :`2` (`self.transition_camera_ref`))) false)
          (goto _label))))
    (:`then_2`
      (bind _aspaper_2dhero (cast `/Game/Blueprints/Hero/Paper2DHero` (`GameplayStatics.GetPlayerPawn` 0)))
      (bind _output_get (set `self.player_ref` _aspaper_2dhero))
      (set `self.hero_camera_ref` (`/Game/Blueprints/Hero/Paper2DHero.hero_camera` _output_get))
      (set `self.hero_flipbook_ref` (`/Game/Blueprints/Hero/Paper2DHero.HeroFlipbook` _output_get))
      (bind _aspaper_2dgame_state_base (cast `/Game/Blueprints/Paper2DGameStateBase` (`GameplayStatics.GetGameState`)))
      (set `self.game_state_ref` _aspaper_2dgame_state_base))
    (:`then_3`
      (bind _output_get_2 (set `self.health` (`/Game/Blueprints/Hero/Paper2DHero.health` _player_ref)))
      (set `self.health_max` _output_get_2)
      (set `self.jump_max` (`/Game/Blueprints/Hero/Paper2DHero.jump_max` _player_ref))
      (set `self.dash_max` (`/Game/Blueprints/Hero/Paper2DHero.dash_max` _player_ref))
      (set `self.jump_velocity` (`/Game/Blueprints/Hero/Paper2DHero.jump_velocity` _player_ref))
      (set `self.dash_velocity` (`/Game/Blueprints/Hero/Paper2DHero.dash_velocity` _player_ref))
      (set `self.detection_stick_size` (+ (.z (`.BoxExtent` (`KismetSystemLibrary.GetComponentBounds` (`Character.CapsuleComponent` _player_ref)))) 20.0)))
    (:`then_4`
      (bind _aspaper_2dhud (cast `/Game/Blueprints/Paper2DHUD` (`self.GetHUD`)))
      (set `self.game_HUD_ref` _aspaper_2dhud))))

(event `MultiJump`
  (bind _player_ref (`self.player_ref`))
  (bind _returnvalue (`self.K2_GetActorLocation` _player_ref))
  (bind _returnvalue_2 (* (`SceneComponent.GetForwardVector` (`/Game/Blueprints/Level/BP_Room.PaperTileMap` (`/Game/Blueprints/Paper2DGameStateBase.room_current` (`self.game_state_ref`)))) (+ (`CapsuleComponent.GetScaledCapsuleRadius` (`Character.CapsuleComponent` _player_ref)) 15.0)))
  ;[0.07248 0.645 0.1291] Jump / Wall Jump
  (if (< (`self.jump_count`) (`self.jump_max`))
    (bind (_outhit _returnvalue_3) (`KismetSystemLibrary.LineTraceSingle` (- _returnvalue _returnvalue_2) (+ _returnvalue _returnvalue_2) "TraceTypeQuery1" true))
    (if _returnvalue_3
      (`self.WallJump` _outhit)
      (else
        (`self.Rejump`)))))

(event `ClimbingEnd`
  (bind _player_ref (`self.player_ref`))
  (bind _charactermovement (`Character.CharacterMovement` _player_ref))
  ;[1 1 1] UNUSE
  ;;[1 1 1] Ladder functions
  (set `/Game/Blueprints/Hero/Paper2DHero.is_climbing` false _player_ref)
  (set `self.can_climb` false)
  (set `self.can_move_horizontaly` true)
  (`PaperFlipbookComponent.SetPlayRate` (`self.hero_flipbook_ref`) 1.0)
  (if (`|EnumEquality` (`CharacterMovementComponent.MovementMode` _charactermovement) "MOVE_Flying")
    (`CharacterMovementComponent.SetMovementMode` _charactermovement "MOVE_Walking" 0)))

(event `UpdateCameraLocation`
  ;[0.6878 0.5153 1] Camera State Machine
  (`self.UseUserCam` 0.0))

(event `Rejump`
  ;[0.07248 0.645 0.1291] Jump / Wall Jump
  (`Character.LaunchCharacter` (`self.player_ref`) (`KismetMathLibrary.MakeVector` 0.0 0.0 (`self.jump_velocity`)) false true :!label _label_2)
  (`/Engine/EditorBlueprintResources/StandardMacros.IncrementInt` (`self.jump_count`) :!label _label_3
    (:`  `
      (`/Game/Blueprints/Hero/Paper2DHero.JumpFX` (`self.player_ref`))
      (`PaperFlipbookComponent.PlayFromStart` (`self.hero_flipbook_ref`)))))

(event `HeroRotationAnimation`
  (bind _capsule_rotation_tmp (`self.capsule_rotation_tmp`))
  (bind _capsulecomponent (`Character.CapsuleComponent` (`self.player_ref`)))
  ;[1 1 1] UNUSE
  ;;[1 1 1] Hero rotation animation
  (set `self.capsule_rotation_tmp` (`SceneComponent.K2_GetComponentRotation` _capsulecomponent))
  (bind (_direction _rotate) (`Timeline|HeroRotationTimeline` :!via `PlayFromStart`)
    (:`Update`
      (`SceneComponent.K2_SetWorldRotation` _capsulecomponent (`KismetMathLibrary.RLerp` _capsule_rotation_tmp (`KismetMathLibrary.MakeRotator` 0.0 0.0 (+ (.yaw _capsule_rotation_tmp) 90.0)) _rotate) false false))
    (:`Finished`
      (`SceneComponent.K2_SetWorldRotation` _capsulecomponent _capsule_rotation_tmp false false))))

(event `ResetCounter`
  ;[1 0.1412 0.2039] Event tick / Reset counter on landing
  (set `self.jump_count` 0)
  (set `self.dash_count` 0))

(event `WallJump`
  (params (Hit :type "HitResult Structure"))
  (bind (_bblockinghit _binitialoverlap _time _location _impactpoint _normal _impactnormal _physmat _hitactor _hitcomponent _hitbonename _hititem _faceindex _tracestart) (`GameplayStatics.BreakHitResult` Hit))
  (bind _hero_flipbook_ref (`self.hero_flipbook_ref`))
  (bind _jump_velocity (`self.jump_velocity`))
  (bind (_returnvalue_x _returnvalue_y) (`KismetMathLibrary.BreakVector` (`self.K2_GetActorLocation` (`self.player_ref`))))
  ;[0.07248 0.645 0.1291] Jump / Wall Jump
  (if (`self.overlap_plateform`)
    (goto _label_2)
    (else
      (`Character.LaunchCharacter` (`self.player_ref`) (`KismetMathLibrary.MakeVector` (* (`KismetMathLibrary.SignOfFloat` (`KismetMathLibrary.Conv_IntToDouble` (`KismetMathLibrary.Round` (- _returnvalue_x (.x _location))))) _jump_velocity) (* (`KismetMathLibrary.SignOfFloat` (`KismetMathLibrary.Conv_IntToDouble` (`KismetMathLibrary.Round` (- _returnvalue_y (.y _location))))) _jump_velocity) _jump_velocity) true true)
      ;;[0.3333 1 0.3608 0.5608] Turn around character
      (if (== _impactpoint _tracestart)
        (`SceneComponent.K2_SetRelativeRotation` _hero_flipbook_ref (struct) false false)
        (goto _label_3)
        (else
          (`SceneComponent.K2_SetRelativeRotation` _hero_flipbook_ref (struct :`Yaw` 180.0) false false)
          (goto _label_3))))))

(event `InputAction|Enter`
  (params (Key :type "Key Structure" :default "AnyKey"))
  ;[0.09412 1 0.8706] UseDoor- GoDown Action / Detect plateform function
  (:`Pressed`
    (if (`self.on_door`)
      (set `self.cam_animation` true)
      (`self.UseTransitionCam`)
      (`self.GoToNextDoor`)
      (`self.UsePursuitCam` (`self.camera_transition_time`))
      (`KismetSystemLibrary.Delay` 0.5)
      (set `self.on_door` true)
      (`KismetSystemLibrary.Delay` 0.5)
      (set `self.cam_animation` false)
      (else
        (`self.CheckUpPlateformCollision` false)))))

(event `self.ReceiveTick`
  (params (DeltaSeconds :type "Float (single-precision)"))
  ;[1 0.1412 0.2039] Event tick / Reset counter on landing
  (`|ExecutionSequence`
    (:`then_0`
      (`self.UpdateCameraLocation`))
    (:`then_1`
      (if (`self.can_climb`)
        _
        (elif (and (`self.up_pressed`) (`self.on_ladder`))
          (set `MovementComponent.Velocity` (0.0 0.0 0.0) (`Character.CharacterMovement` (`self.player_ref`)))
          (set `self.can_climb` true))))
    (:`then_2`
      (if (`/Game/Blueprints/Hero/Paper2DHero.is_jumping` (`self.player_ref`))
        (`self.CheckUpPlateformCollision` true)))))

(event `CheckUpPlateformCollision`
  (params (Up :type Boolean))
  (bind _returnvalue (`SceneComponent.K2_GetComponentLocation` (`Character.CapsuleComponent` (`self.player_ref`))))
  ;[0.09412 1 0.8706] UseDoor- GoDown Action / Detect plateform function
  (bind _outhit (`KismetSystemLibrary.LineTraceSingle` _returnvalue (`KismetMathLibrary.MakeVector` (.x _returnvalue) (.y _returnvalue) (+ (.z _returnvalue) (* (`self.detection_stick_size`) (select `bool` Up :`false` -1.0 :`true` 1.0 :!type "Float (single-precision)")))) "TraceTypeQuery1"))
  (bind _asbp_plateform (cast `/Game/Blueprints/Level/BP_Plateform` (`.HitActor` (`GameplayStatics.BreakHitResult` _outhit))))
  (`PrimitiveComponent.SetCollisionResponseToChannel` (`/Game/Blueprints/Level/BP_Plateform.Box` _asbp_plateform) "ECC_Pawn" "ECR_Overlap"))

(event `InputAction|RightDash`
  (params (Key :type "Key Structure" :default "AnyKey"))
  (bind _player_ref (`self.player_ref`))
  ;[0.07248 0.645 0.1291] Dash
  (:`Pressed`
    (if (< (`self.dash_count`) (`self.dash_max`))
      (`Character.LaunchCharacter` (`self.player_ref`) (`KismetMathLibrary.GreaterGreater_VectorRotator` (`KismetMathLibrary.MakeVector` (`self.dash_velocity`) 0.0 100.0) (`SceneComponent.K2_GetComponentRotation` (`/Game/Blueprints/Level/BP_Room.PaperTileMap` (`/Game/Blueprints/Paper2DGameStateBase.room_current` (`self.game_state_ref`))))) true true)
      (`/Engine/EditorBlueprintResources/StandardMacros.IncrementInt` (`self.dash_count`) :!label _label_4
        (:`  `
          (`/Game/Blueprints/Hero/Paper2DHero.JumpFX` _player_ref)
          (set `/Game/Blueprints/Hero/Paper2DHero.is_dashing` true _player_ref)
          (`KismetSystemLibrary.Delay` 0.8)
          (set `/Game/Blueprints/Hero/Paper2DHero.is_dashing` false _player_ref))))))

(event `UseUserCam`
  (params (duration :type "Float (double-precision)"))
  ;[0.6878 0.5153 1] Set current view to hero / pursuit / transition camera
  (`self.SetViewTargetWithBlend` (`self.player_ref`) 0.0))

(event `UsePursuitCam`
  (params (blend_time :type "Float (double-precision)"))
  ;[0.6878 0.5153 1] Set current view to hero / pursuit / transition camera
  (`SceneComponent.K2_SetWorldRotation` (`CameraActor.CameraComponent` (`self.pursuit_camera_ref`)) (`SceneComponent.K2_GetComponentRotation` (`self.hero_camera_ref`)) false false)
  (`self.SetViewTargetWithBlend` (`self.pursuit_camera_ref`) blend_time "VTBlend_Linear" 0.0 true))

(event `InputAction|LeftDash`
  (params (Key :type "Key Structure" :default "AnyKey"))
  ;[0.07248 0.645 0.1291] Dash
  (:`Pressed`
    (if (< (`self.dash_count`) (`self.dash_max`))
      (`Character.LaunchCharacter` (`self.player_ref`) (`KismetMathLibrary.GreaterGreater_VectorRotator` (`KismetMathLibrary.MakeVector` (- 0.0 (`self.dash_velocity`)) 0.0 100.0) (`SceneComponent.K2_GetComponentRotation` (`/Game/Blueprints/Level/BP_Room.PaperTileMap` (`/Game/Blueprints/Paper2DGameStateBase.room_current` (`self.game_state_ref`))))) true true)
      (goto _label_4))))

(event `UseTransitionCam`
  (bind _cameracomponent (`CameraActor.CameraComponent` (`self.transition_camera_ref`)))
  (bind _cameracomponent_2 (`CameraActor.CameraComponent` (`self.pursuit_camera_ref`)))
  ;[0.6878 0.5153 1] Set current view to hero / pursuit / transition camera
  (`SceneComponent.K2_SetWorldRotation` _cameracomponent (`SceneComponent.K2_GetComponentRotation` _cameracomponent_2) false false)
  (`SceneComponent.K2_SetWorldLocation` _cameracomponent (`SceneComponent.K2_GetComponentLocation` _cameracomponent_2) false false)
  (`self.SetViewTargetWithBlend` (`self.transition_camera_ref`) 0.0 "VTBlend_Linear" 0.0))

(event `Key|R`
  (params (Key :type "Key Structure" :default "AnyKey")))

(fn `GoToNextDoor`
  (bind _player_ref (`self.player_ref`))
  (bind _game_state_ref (`self.game_state_ref`))
  (bind _world_map (`/Game/Blueprints/Paper2DGameStateBase.world_map` _game_state_ref))
  (bind _next_door_ref (`/Game/Blueprints/Level/BP_Door.next_door_ref` (`self.current_door`)))
  (bind _world_id (`/Game/Blueprints/Level/BP_Door.world_id` _next_door_ref))
  (bind _returnvalue (`SceneComponent.K2_GetComponentRotation` (`/Game/Blueprints/Level/BP_Door.DefaultSceneRoot` (`/Game/Blueprints/Level/BP_Door.next_door_ref` (`self.current_door`)))))
  (`|ExecutionSequence`
    (:`then_1`
      (`/Game/Blueprints/Level/BP_World.SetWorldVisible` (`BlueprintMapLibrary.Map_Find` _world_map (`/Game/Blueprints/Paper2DGameStateBase.current_world_id` _game_state_ref)) false)
      (`/Game/Blueprints/Level/BP_World.SetWorldVisible` (`BlueprintMapLibrary.Map_Find` _world_map _world_id) true)
      (`/Game/Blueprints/Paper2DGameStateBase.UpdateCurrentRoom` _game_state_ref _world_id (`/Game/Blueprints/Level/BP_Door.room_id` _next_door_ref)))
    (:`then_2`
      (`SceneComponent.K2_SetWorldRotation` (`PaperCharacter.Sprite` _player_ref) _returnvalue false false)
      (`SceneComponent.K2_SetWorldRotation` (`/Game/Blueprints/Hero/Paper2DHero.SpringArm` _player_ref) (`KismetMathLibrary.MakeRotator` (.roll _returnvalue) (.pitch _returnvalue) (+ (.yaw _returnvalue) 90.0)) false false))
    (:`then_3`
      (`SceneComponent.K2_SetWorldLocation` (`Character.CapsuleComponent` (`self.player_ref`)) (`self.K2_GetActorLocation` (`/Game/Blueprints/Level/BP_Door.next_door_ref` (`self.current_door`))) false true))))

(fn `GoToWorldSpawn`
  (params (spawn :type "/Game/Blueprints/Level/BP_Spawner Object Reference"))
  (returns (world_id :type Integer) (room_id :type Integer))
  (bind _player_ref (`self.player_ref`))
  (bind _returnvalue (`SceneComponent.K2_GetComponentRotation` (`/Game/Blueprints/Level/BP_Spawner.DefaultSceneRoot` spawn)))
  (`|ExecutionSequence`
    (:`then_0`
      (`SceneComponent.K2_SetWorldRotation` (`PaperCharacter.Sprite` _player_ref) _returnvalue false false)
      (`SceneComponent.K2_SetWorldRotation` (`/Game/Blueprints/Hero/Paper2DHero.SpringArm` _player_ref) (`KismetMathLibrary.MakeRotator` (.roll _returnvalue) (.pitch _returnvalue) (+ (.yaw _returnvalue) 90.0)) false false))
    (:`then_1`
      (`SceneComponent.K2_SetWorldLocation` (`Character.CapsuleComponent` (`self.player_ref`)) (`self.K2_GetActorLocation` spawn) false true))
    (:`then_2`
      (return (`/Game/Blueprints/Level/BP_Spawner.world_id` spawn) (`/Game/Blueprints/Level/BP_Spawner.room_id` spawn)))))

(fn `OnDamage`
  (bind _player_ref (`self.player_ref`))
  (if (not (`/Game/Blueprints/Hero/Paper2DHero.is_invisible` _player_ref))
    (`GameplayStatics.ApplyDamage` _player_ref 1.0)
    (`|ExecutionSequence`
      (:`then_0`
        (set `/Game/Blueprints/Hero/Paper2DHero.is_invisible` true (`self.player_ref`)))
      (:`then_1`
        (if (`self.has_mushroom`)
          (`/Game/Blueprints/Hero/Paper2DHero.ScaleControle` _player_ref false)
          (else
            (`/Engine/EditorBlueprintResources/StandardMacros.DecrementInt` (`self.health`)
              (:`  `
                (`/Game/Blueprints/HUD/PaperGameHUD.UpdateHealth` (`/Game/Blueprints/Paper2DHUD.player_HUD_ref` (`self.game_HUD_ref`)))
                (set `/Game/Blueprints/Hero/Paper2DHero.is_damaged` true (`self.player_ref`))))))))))

(fn `OnPickUp`
  (params (ItemType :type "/Game/Blueprints/PickUp/BP_PickUpBase Object Reference"))
  (cast `/Game/Blueprints/PickUp/BP_PickUpMushroom` ItemType
    (:`then`
      (set `self.has_mushroom` true)
      (`/Game/Blueprints/Hero/Paper2DHero.ScaleControle` (`self.player_ref`) true))
    (:`CastFailed`
      (cast `/Game/Blueprints/PickUp/BP_PickUp_Ring` ItemType
        (:`then`
          (`/Engine/EditorBlueprintResources/StandardMacros.IncrementInt` (`self.ring_collected`)))
        (:`CastFailed`
          (cast `/Game/Blueprints/PickUp/BP_PickUp_Health` ItemType)
          (if (< (`self.health`) (`self.health_max`))
            (`/Engine/EditorBlueprintResources/StandardMacros.IncrementInt` (`self.health`)
              (:`  `
                (`/Game/Blueprints/HUD/PaperGameHUD.UpdateHealth` (`/Game/Blueprints/Paper2DHUD.player_HUD_ref` (`self.game_HUD_ref`)))))))))))

(fn `UserConstructionScript`)