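; Player character Blueprint for a 2D Paper2D platformer, handling animation, projectile firing, damage knockback and mushroom-driven size changes.
; Each tick, movement and state flags feed a prioritized state machine that picks the hero's flipbook.
; Room collision overlaps pass doors to the player controller and rooms to the game state, which recomputes camera limits.
; Dust emitters serve jump and landing effects; dash/jump squash timelines are unconnected.
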(event `InputAction|Fire`
  (params (Key :type "Key Structure" :default "AnyKey"))
  ;[0.07248 0.645 0.1291] Fire Input / Launch Projectile
  (:`Pressed`
    (set `self.is_attacking` true)
    (`self.FireProjectile`)))

(event `JumpFX`
  ;[0.1922 0.4588 1] Jump/Dash effect
  (`GameplayStatics.SpawnEmitterAtLocation` "/Game/Particles/pDust.pDust" (`SceneComponent.K2_GetComponentLocation` (`self.DustBox`))))

(event `self.ReceiveBeginPlay`
  ;[1 0.1412 0.2039] Event Begin Play
  (`KismetSystemLibrary.PrintString` "[PAPER2DHERO]")
  (bind _aspaper_2dcontroller (cast `/Game/Blueprints/Paper2DController` (`GameplayStatics.GetPlayerController` 0)))
  (set `self.player_controller_ref` _aspaper_2dcontroller)
  (bind _aspaper_2dgame_state_base (cast `/Game/Blueprints/Paper2DGameStateBase` (`GameplayStatics.GetGameState`)))
  (set `self.game_state_ref` _aspaper_2dgame_state_base))

(event `FireProjectile`
  ;[0.07248 0.645 0.1291] Fire Input / Launch Projectile
  (`|SpawnActorFromClass` "/Game/Blueprints/BP_Projectile.BP_Projectile_C" (`SceneComponent.K2_GetComponentToWorld` (`self.ProjectileSpawn`)) "AlwaysSpawn" "OverrideRootScale")
  (set `self.is_attacking` false))

(event `LandFX`
  ;[0.1922 0.4588 1] Jump/Dash effect
  (`GameplayStatics.SpawnEmitterAtLocation` "/Game/Particles/pDust.pDust" (`SceneComponent.K2_GetComponentLocation` (`self.DustBox`))))

(event `self.ReceiveTick`
  (params (DeltaSeconds :type "Float (single-precision)"))
  ;[1 0.1412 0.2039] Event Begin Play
  (`self.UpdateAnimation`))

(event `self.OnLanded`
  (params (Hit :type "HitResult Structure (by ref)"))
  ;[1 0.1412 0.2039] Collision Room
  (`/Game/Blueprints/Paper2DController.ResetCounter` (`self.player_controller_ref`))
  (set `self.is_damaged` false))

(event `ScaleControle`
  (params (is_health :type Boolean))
  ;[0.1922 0.4588 1] Mushroom effect / Health size swap
  (if is_health
    (if (`/Game/Blueprints/Paper2DController.has_mushroom` (`self.player_controller_ref`))
      (bind (_direction _scalelerp) (`Timeline|scale_timeline` :!via `PlayFromStart`)
        (:`Update`
          (`self.SetActorScale3D` _scalelerp)
          (set `self.current_scale` (`self.increased_scale`)))))
    (else
      (bind (_direction_2 _scalelerp_2) (`Timeline|scale_end_timeline` :!via `PlayFromStart`)
        (:`Update`
          (`self.SetActorScale3D` _scalelerp_2)
          (set `self.current_scale` (`self.start_scale`))
          (set `/Game/Blueprints/Paper2DController.has_mushroom` false (`self.player_controller_ref`)))))))

(event `self.RoomCollision.OnComponentBeginOverlap`
  (params (OverlappedComponent :type "PrimitiveComponent Object Reference") (OtherActor :type "Actor Object Reference") (OtherComp :type "PrimitiveComponent Object Reference") (OtherBodyIndex :type Integer) (bFromSweep :type Boolean) (SweepResult :type "HitResult Structure (by ref)"))
  (bind _player_controller_ref (`self.player_controller_ref`))
  ;[1 0.1412 0.2039] Collision Room
  (`/Engine/EditorBlueprintResources/StandardMacros.IsValid` _player_controller_ref
    (:`Is Valid`
      (bind _asbp_door (cast `/Game/Blueprints/BP_Door` OtherActor)
        (:`then`
          (set `/Game/Blueprints/Paper2DController.current_door` _asbp_door _player_controller_ref))
        (:`CastFailed`
          (bind _asbp_room (cast `/Game/Blueprints/BP_Room` OtherActor))
          (`/Game/Blueprints/Paper2DGameStateBase.UpdateCurrentRoomInfos` (`self.game_state_ref`) (`/Game/Blueprints/BP_Room.world_id` _asbp_room) (`/Game/Blueprints/BP_Room.room_id` _asbp_room))
          (`/Game/Blueprints/Paper2DGameStateBase.ComputeCameraLimit` (`self.game_state_ref`)))))))

(event `self.RoomCollision.OnComponentEndOverlap`
  (params (OverlappedComponent :type "PrimitiveComponent Object Reference") (OtherActor :type "Actor Object Reference") (OtherComp :type "PrimitiveComponent Object Reference") (OtherBodyIndex :type Integer))
  ;[1 0.1412 0.2039] Collision Room
  (cast `/Game/Blueprints/BP_Room` OtherActor))

(event `self.ReceiveAnyDamage`
  (params (Damage :type "Float (single-precision)") (DamageType :type "DamageType Object Reference") (InstigatedBy :type "Controller Object Reference") (DamageCauser :type "Actor Object Reference"))
  ;[0.1922 0.4588 1] Damage impulse
  (`self.LaunchCharacter` (`KismetMathLibrary.GreaterGreater_VectorRotator` (`KismetMathLibrary.GreaterGreater_VectorRotator` (`KismetMathLibrary.MakeVector` -400.0 0.0 600.0) (`SceneComponent.K2_GetComponentRotation` (`self.Sprite`))) (`SceneComponent.RelativeRotation` (`self.HeroFlipbook`))) true true)
  (`KismetSystemLibrary.Delay` 2.0)
  (set `self.is_invisible` false))

(event `UpdateAnimation`
  (bind _returnvalue (`KismetMathLibrary.VSize` (`self.GetVelocity`)))
  ;[0.6878 0.5153 1] Animation State Machine
  (set `self.is_moving` (> _returnvalue 0.0))
  (set `self.is_falling` (> _returnvalue 1450.0))
  (set `self.is_start_falling` (< (.z (`self.GetVelocity`)) 0.0))
  (set `self.is_jumping` (`NavMovementComponent.IsFalling` (`self.CharacterMovement`)))
  (bind _flipbook (`self.AnimationStateMachine`))
  (`PaperFlipbookComponent.SetFlipbook` (`self.HeroFlipbook`) _flipbook))

(fn `AnimationStateMachine`
  (returns (FlipBook :type "PaperFlipbook Object Reference"))
  (locals (animation_state :type "/Game/Data/AnimationState Enum"))
  (if (`self.is_dashing`)
    (set `local.animation_state` "NewEnumerator3")
    (elif (`self.is_climbing`)
      (set `local.animation_state` "NewEnumerator7")
      (elif (`self.is_attacking`)
        (set `local.animation_state` "NewEnumerator4")
        (elif (`self.is_damaged`)
          (set `local.animation_state` "NewEnumerator8")
          (elif (`self.is_falling`)
            (set `local.animation_state` "NewEnumerator5")
            (elif (`self.is_start_falling`)
              (set `local.animation_state` "NewEnumerator6")
              (elif (`self.is_jumping`)
                (set `local.animation_state` "NewEnumerator2")
                (elif (`self.is_moving`)
                  (set `local.animation_state` "NewEnumerator1")
                  (else
                    (set `local.animation_state` "NewEnumerator0"))))))))))
  (return (select `/Game/Data/AnimationState` (`local.animation_state`) :`NewEnumerator0` "/Game/Animations/hero_idle.hero_idle" :`NewEnumerator1` "/Game/Animations/hero_run.hero_run" :`NewEnumerator2` "/Game/Animations/jump_start.jump_start" :`NewEnumerator3` "/Game/Animations/jump_start.jump_start" :`NewEnumerator6` "/Game/Animations/jump_fall1.jump_fall1" :`NewEnumerator5` "/Game/Animations/jump_fall2.jump_fall2" :`NewEnumerator7` "/Game/Animations/hero_run.hero_run" :`NewEnumerator8` "/Game/Animations/hero_damage.hero_damage" :!type "PaperFlipbook Object Reference")))

(fn `UserConstructionScript`
  (set `CharacterMovementComponent.JumpZVelocity` (`self.jump_velocity`) (`self.CharacterMovement`))
  (set `self.JumpMaxHoldTime` 0.5)
  (bind _output_get (set `self.start_scale` (`self.GetActorScale3D`)))
  (set `self.current_scale` _output_get))