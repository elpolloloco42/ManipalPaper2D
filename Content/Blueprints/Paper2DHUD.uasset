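; HUD class for a Paper2D game that manages the lobby, player and respawn screens.
; On BeginPlay it creates the three widgets, registers itself with the Paper2D player controller and shows the lobby.
; SetHUD swaps the current widget in the viewport, then ChangeControl toggles the cursor and input mode: UI-only for lobby and respawn, game-only for the player HUD.
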(event `self.ReceiveBeginPlay`
  ;[1 0.121 0.2007] BeginPlay
  (`|ExecutionSequence`
    (:`then_0`
      (bind _returnvalue (`|CreateWidget` "/Game/UI/HUD_Player.HUD_Player_C"))
      (set `self.player_HUD` _returnvalue)
      (bind _returnvalue_2 (`|CreateWidget` "/Game/UI/Lobby/HUD_Lobby.HUD_Lobby_C"))
      (set `self.lobby_HUD` _returnvalue_2)
      (bind _returnvalue_3 (`|CreateWidget` "/Game/UI/Respawn/HUD_Respawn.HUD_Respawn_C"))
      (set `self.respawn_HUD_ref` _returnvalue_3))
    (:`then_1`
      (bind _aspaper_2dplayer_controller (cast `/Game/Blueprints/Gameplay/Paper2DPlayerController` (`GameplayStatics.GetPlayerController` 0)))
      (bind _output_get (set `self.player_controller_ref` _aspaper_2dplayer_controller))
      (set `/Game/Blueprints/Gameplay/Paper2DPlayerController.HUD_ref` self _output_get))
    (:`then_2`
      (`self.SetHUD` "NewEnumerator2"))))

(event `SetHUD`
  (params (NewHUD :type "/Game/Data/E_HUD Enum"))
  (bind _current_hud (`self.current_HUD`))
  (bind _returnvalue (select `/Game/Data/E_HUD` NewHUD :`NewEnumerator0` (`self.player_HUD`) :`NewEnumerator1` (`self.respawn_HUD`) :`NewEnumerator2` (`self.lobby_HUD`) :!type "UserWidget Object Reference"))
  ;[0.3059 1 0.2732] Change Current HUD
  (`|ExecutionSequence`
    (:`then_0`
      (`/Engine/EditorBlueprintResources/StandardMacros.IsValid` _current_hud
        (:`Is Valid`
          (`Widget.RemoveFromParent` _current_hud))))
    (:`then_1`
      (`UserWidget.AddToViewport` _returnvalue 0)
      (set `self.current_HUD` _returnvalue))
    (:`then_2`
      (`self.ChangeControl` (select `/Game/Data/E_HUD` NewHUD :`NewEnumerator1` true :`NewEnumerator2` true)))))

(event `ChangeControl`
  (params (`UI Mode` :type Boolean))
  (bind _player_controller_ref (`self.player_controller_ref`))
  ;[0.3059 1 0.2732] Set Control To UI / Game Only
  (set `PlayerController.bShowMouseCursor` `UI Mode` (`self.player_controller_ref`))
  (if `UI Mode`
    (`WidgetBlueprintLibrary.SetInputMode_UIOnlyEx` _player_controller_ref (`self.current_HUD`))
    (else
      (`WidgetBlueprintLibrary.SetInputMode_GameOnly` _player_controller_ref))))

(fn `UserConstructionScript`)