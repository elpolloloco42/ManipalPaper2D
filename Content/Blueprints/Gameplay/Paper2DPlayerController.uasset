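; Player controller for a networked Paper2D platformer that spawns, possesses and respawns the player's hero at its assigned spawn point.
; Forwards move, fire, jump, dash, platform and door input to the hero, mostly gated by player-state checks.
; Relays lobby name and ready changes to the game mode.
; Applies ring, mushroom and health pickups to player state, splitting transforms and effects to authority and HUD updates to remote.
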(event `Spawn`
  (params (id :type Integer) (name :type Text))
  ;[0.7682 0.4567 1] [SERVER] Spawn Hero
  (bind _outactors (`GameplayStatics.GetAllActorsOfClass` "/Game/Blueprints/Level/Paper2D_LevelBlueprint.Paper2D_LevelBlueprint_C"))
  (bind _spawn (`/Game/Blueprints/Level/BP_World.spawn` (`BlueprintMapLibrary.Map_Find` (`/Game/Blueprints/Level/Paper2D_LevelBlueprint.world_map` (`KismetArrayLibrary.Array_Get` _outactors)) id)))
  (bind _returnvalue (`|SpawnActorFromClass` "/Game/Blueprints/Characters/Hero/Paper2DHero.Paper2DHero_C" (`self.GetTransform` _spawn) "Undefined" "OverrideRootScale" null id name))
  (set `self.spawn_ref` _spawn)
  (`self.Possess` _returnvalue))

(event `ChangeName`
  (params (name :type Text))
  (bind _game_mode_ref (`self.game_mode_ref`))
  ;[0.7682 0.4567 1] [SERVER] HUD Lobby - Call Changing Event
  (`/Engine/EditorBlueprintResources/StandardMacros.IsValid` _game_mode_ref
    (:`Is Valid`
      (`/Game/Blueprints/Gameplay/Paper2DGameMode.SetPlayerName` _game_mode_ref name (`self.player_id`)))))

(event `InputAxis|HonrizontalMove`
  (params (AxisValue :type "Float (single-precision)"))
  (bind _paper_hero_ref (`self.paper_hero_ref`))
  (bind _player_state_ref (`/Game/Blueprints/Characters/Hero/Paper2DHero.player_state_ref` (`self.paper_hero_ref`)))
  ;[0.7682 0.4567 1] [SERVER] All Input Call
  (if (`self.start`)
    (`/Engine/EditorBlueprintResources/StandardMacros.IsValid` _player_state_ref
      (:`Is Valid`
        (if (not (`/Game/Blueprints/Paper2DPlayerState.is_dead` _player_state_ref))
          (`/Game/Blueprints/Characters/Hero/Paper2DHero.CheckRotationFlipbook` _paper_hero_ref AxisValue)
          (`Pawn.AddMovementInput` _paper_hero_ref (`SceneComponent.GetForwardVector` (`Character.CapsuleComponent` _paper_hero_ref)) AxisValue false))))))

(event `self.ReceiveBeginPlay`
  ;[1 0.121 0.2007] BeginPlay Even Tick
  (`self.SetActorTickEnabled` true)
  (bind _aspaper_2dgame_mode (cast `/Game/Blueprints/Gameplay/Paper2DGameMode` (`GameplayStatics.GetGameMode`)))
  (set `self.game_mode_ref` _aspaper_2dgame_mode))

(event `self.ReceiveTick`
  (params (DeltaSeconds :type "Float (single-precision)"))
  ;[1 0.121 0.2007] BeginPlay Even Tick
  (`/Engine/EditorBlueprintResources/StandardMacros.DoOnce` false :!label _label
    (:`Completed`
      (bind _aspaper_2dgame_state (cast `/Game/Blueprints/Paper2DGameState` (`GameplayStatics.GetGameState`))
        (:`then`
          (set `self.game_state_ref` _aspaper_2dgame_state))
        (:`CastFailed`
          (goto _label :!via `Reset`))))))

(event `ChangePlayerReady`
  (params (ready :type Boolean))
  (bind _game_mode_ref (`self.game_mode_ref`))
  ;[0.7682 0.4567 1] [SERVER] HUD Lobby - Call Changing Event
  (`/Engine/EditorBlueprintResources/StandardMacros.IsValid` _game_mode_ref
    (:`Is Valid`
      (`/Game/Blueprints/Gameplay/Paper2DGameMode.SetPlayerReady` _game_mode_ref ready (`self.player_id`)))))

(event `InputAction|fire`
  (params (Key :type "Key Structure" :default "AnyKey"))
  (bind _paper_hero_ref (`self.paper_hero_ref`))
  ;[0.7682 0.4567 1] [SERVER] All Input Call
  (:`Pressed`
    (if (not (`/Game/Blueprints/Paper2DPlayerState.is_damaged` (`/Game/Blueprints/Characters/Hero/Paper2DHero.player_state_ref` _paper_hero_ref)))
      (`/Game/Blueprints/Characters/Hero/Paper2DHero.FireAction` _paper_hero_ref))))

(event `InputAction|Jump`
  (params (Key :type "Key Structure" :default "AnyKey"))
  (bind _paper_hero_ref (`self.paper_hero_ref`))
  ;[0.7682 0.4567 1] [SERVER] All Input Call
  (:`Pressed`
    (if (not (`/Game/Blueprints/Paper2DPlayerState.is_damaged` (`/Game/Blueprints/Characters/Hero/Paper2DHero.player_state_ref` (`self.paper_hero_ref`))))
      (`/Game/Blueprints/Characters/Hero/Paper2DHero.JumpAction` _paper_hero_ref)))
  (:`Released`
    (`Character.StopJumping` _paper_hero_ref)))

(event `Respawn`
  ;[0.7682 0.4567 1] [SERVER] Respawn
  (`self.RespawnEvent`))

(event `InputAction|LeftDash`
  (params (Key :type "Key Structure" :default "AnyKey"))
  ;[0.7682 0.4567 1] [SERVER] All Input Call
  (:`Pressed`
    (if (not (`/Game/Blueprints/Paper2DPlayerState.is_damaged` (`/Game/Blueprints/Characters/Hero/Paper2DHero.player_state_ref` (`self.paper_hero_ref`))))
      (`/Game/Blueprints/Characters/Hero/Paper2DHero.DashAction` (`self.paper_hero_ref`) false))))

(event `InputAction|PlateformAction`
  (params (Key :type "Key Structure" :default "AnyKey"))
  ;[0.7682 0.4567 1] [SERVER] All Input Call
  (:`Pressed`
    (if (not (`/Game/Blueprints/Paper2DPlayerState.is_damaged` (`/Game/Blueprints/Characters/Hero/Paper2DHero.player_state_ref` (`self.paper_hero_ref`))))
      (`/Game/Blueprints/Characters/Hero/Paper2DHero.PlateformAction` (`self.paper_hero_ref`) false))))

(event `InitPlayerHUD`
  (bind _hud_ref (`self.HUD_ref`))
  (bind _player_hud (`/Game/Blueprints/Paper2DHUD.player_HUD` _hud_ref))
  ;[0.1816 0.351 1] [ON EACH] HUD Player - Init
  (`/Engine/EditorBlueprintResources/StandardMacros.IsValid` _hud_ref
    (:`Is Valid`
      (set `/Game/UI/HUD_Player.player_ref` (`self.paper_hero_ref`) _player_hud)
      (`/Game/UI/HUD_Player.InitHealth` _player_hud)
      (`/Game/Blueprints/Paper2DHUD.SetHUD` (`self.HUD_ref`) "NewEnumerator0"))))

(event `InputAction|RightDash`
  (params (Key :type "Key Structure" :default "AnyKey"))
  ;[0.7682 0.4567 1] [SERVER] All Input Call
  (:`Pressed`
    (if (not (`/Game/Blueprints/Paper2DPlayerState.is_damaged` (`/Game/Blueprints/Characters/Hero/Paper2DHero.player_state_ref` (`self.paper_hero_ref`))))
      (`/Game/Blueprints/Characters/Hero/Paper2DHero.DashAction` (`self.paper_hero_ref`) true))))

(event `InputAction|DoorAction`
  (params (Key :type "Key Structure" :default "AnyKey"))
  ;[0.7682 0.4567 1] [SERVER] All Input Call
  (:`Pressed`
    (if (not (`/Game/Blueprints/Paper2DPlayerState.is_damaged` (`/Game/Blueprints/Characters/Hero/Paper2DHero.player_state_ref` (`self.paper_hero_ref`))))
      (`/Game/Blueprints/Characters/Hero/Paper2DHero.DoorAction` (`self.paper_hero_ref`)))))

(event `RespawnEvent`
  (bind _paper_hero_ref (`self.paper_hero_ref`))
  (bind _hud_ref (`self.HUD_ref`))
  ;[0.1816 0.351 1] [ON EACH] Respawn / Set Location to Spawn / Set Player HUD
  (`/Game/Blueprints/Paper2DPlayerState.InitSpecs` (`/Game/Blueprints/Characters/Hero/Paper2DHero.player_state_ref` _paper_hero_ref) _paper_hero_ref)
  (`/Game/Blueprints/Characters/Hero/Paper2DHero.ChangeOverlap` _paper_hero_ref false)
  (`/Engine/EditorBlueprintResources/ActorMacros.Switch Has Authority`
    (:`Authority`
      (`SceneComponent.K2_SetWorldTransform` (`Character.CapsuleComponent` (`self.paper_hero_ref`)) (`self.GetTransform` (`self.spawn_ref`)) false false))
    (:`Remote`
      (`/Game/Blueprints/Paper2DHUD.SetHUD` _hud_ref "NewEnumerator0")
      (`/Game/UI/HUD_Player.UpdateHealth` (`/Game/Blueprints/Paper2DHUD.player_HUD` _hud_ref)))))

(event `OnPickUp`
  (params (item :type "/Game/Blueprints/PickUp/BP_PickUpBase Object Reference"))
  (bind _paper_hero_ref (`self.paper_hero_ref`))
  (bind _paper_hero_ref_2 (`self.paper_hero_ref`))
  (bind _player_state_ref (`/Game/Blueprints/Characters/Hero/Paper2DHero.player_state_ref` _paper_hero_ref_2))
  (bind _health (`/Game/Blueprints/Paper2DPlayerState.health` (`/Game/Blueprints/Characters/Hero/Paper2DHero.player_state_ref` _paper_hero_ref)))
  ;[0.3059 1 0.2732] On PickUp
  (cast `/Game/Blueprints/PickUp/BP_PickUp_Ring` item
    (:`then`
      (`/Engine/EditorBlueprintResources/StandardMacros.IncrementInt` (`/Game/Blueprints/Paper2DPlayerState.ring_collected` (`/Game/Blueprints/Characters/Hero/Paper2DHero.player_state_ref` (`self.paper_hero_ref`)))))
    (:`CastFailed`
      (cast `/Game/Blueprints/PickUp/BP_PickUpMushroom` item
        (:`then`
          (if (not (`/Game/Blueprints/Paper2DPlayerState.has_mushroom` _player_state_ref))
            (set `/Game/Blueprints/Paper2DPlayerState.has_mushroom` true _player_state_ref)
            (`/Engine/EditorBlueprintResources/ActorMacros.Switch Has Authority`
              (:`Authority`
                (`/Game/Blueprints/Characters/Hero/Paper2DHero.ApplyMushroomEffect` _paper_hero_ref_2 true)))))
        (:`CastFailed`
          (cast `/Game/Blueprints/PickUp/BP_PickUp_Health` item)
          (if (< _health (`/Game/Blueprints/Characters/Hero/Paper2DHero.health` _paper_hero_ref))
            (`/Engine/EditorBlueprintResources/StandardMacros.IncrementInt` _health
              (:`  `
                (`/Engine/EditorBlueprintResources/ActorMacros.Switch Has Authority`
                  (:`Remote`
                    (`/Game/UI/HUD_Player.UpdateHealth` (`/Game/Blueprints/Paper2DHUD.player_HUD` (`self.HUD_ref`)))))))))))))

(fn `UserConstructionScript`)