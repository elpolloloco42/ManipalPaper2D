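; Paper2D multiplayer game mode that manages lobby players and their spawning.
; On post-login it registers each controller, assigns an index-based ID and name, and adds an entry to the Paper2D game state.
; Name and ready changes forward to the game state.
; Readying up spawns every registered controller immediately, as the all-players-ready comparison is left unconnected.
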(event `self.ReceiveBeginPlay`
  ;[1 0.121 0.2007] BeginPlay / OnPostLogin
  (bind _aspaper_2dgame_state (cast `/Game/Blueprints/Paper2DGameState` (`GameplayStatics.GetGameState`)))
  (set `self.game_state_ref` _aspaper_2dgame_state))

(event `SetPlayerReady`
  (params (ready :type Boolean) (id :type Integer))
  ;[0.7682 0.4567 1] LobbyHUD Changing Event / Check for Spawn
  (`|ExecutionSequence`
    (:`then_0`
      (`/Game/Blueprints/Paper2DGameState.UpdatePlayerStatus` (`self.game_state_ref`) ready id))
    (:`then_1`
      (`self.SpawnPlayers` ready))))

(event `self.K2_PostLogin`
  (params (NewPlayer :type "PlayerController Object Reference"))
  ;[1 0.121 0.2007] BeginPlay / OnPostLogin
  (bind _aspaper_2dplayer_controller (cast `/Game/Blueprints/Gameplay/Paper2DPlayerController` NewPlayer))
  (`self.InitPlayerControllerInfo` _aspaper_2dplayer_controller))

(event `SetPlayerName`
  (params (name :type Text) (id :type Integer))
  ;[0.7682 0.4567 1] LobbyHUD Changing Event / Check for Spawn
  (`/Game/Blueprints/Paper2DGameState.UpdatePlayerName` (`self.game_state_ref`) name id))

(event `InitPlayerControllerInfo`
  (params (player_controller :type "/Game/Blueprints/Gameplay/Paper2DPlayerController Object Reference"))
  ;[0.7682 0.4567 1] Set Player Controller Infos
  (bind _returnvalue (`KismetArrayLibrary.Array_Add` (`self.player_controllers_ref`) player_controller))
  (set `/Game/Blueprints/Gameplay/Paper2DPlayerController.player_id` _returnvalue player_controller)
  (bind _output_get (set `/Game/Blueprints/Gameplay/Paper2DPlayerController.Name` (`KismetTextLibrary.Conv_StringToText` (`KismetStringLibrary.Concat_StrStr` (`KismetTextLibrary.Conv_TextToString` (`/Game/Blueprints/Gameplay/Paper2DPlayerController.Name` player_controller)) (`KismetStringLibrary.Conv_IntToString` _returnvalue))) player_controller))
  (`/Game/Blueprints/Paper2DGameState.AddInfos` (`self.game_state_ref`) (make `/Game/Data/S_PlayerInfos` _output_get)))

(event `SpawnPlayers`
  (params (ready :type Boolean))
  (bind _ready (`self.ready`))
  ;[0.7682 0.4567 1] Spawn Players When All Are Ready
  (if ready
    (bind _result (`/Engine/EditorBlueprintResources/StandardMacros.IncrementInt` _ready)
      (:`  `
        (if true
          (for (_array_element _array_index) (`self.player_controllers_ref`)
            (`/Game/Blueprints/Gameplay/Paper2DPlayerController.Spawn` _array_element _array_index "")))))
    (else
      (`/Engine/EditorBlueprintResources/StandardMacros.DecrementInt` _ready))))

(fn `UserConstructionScript`)