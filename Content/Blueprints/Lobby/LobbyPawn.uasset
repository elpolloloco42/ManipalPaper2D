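; Lobby player character: a Paper2D flipbook hero in a random color that runs, multi-jumps, wall-jumps, dashes and fires projectiles.
; Tick derives movement flags and feeds a priority-based state machine that swaps flipbooks from the color's animation set.
; Jumps and dashes use capped launches reset on landing, with a line trace choosing wall jump or rejump.
; Damage triggers knockback and timed invincibility, altering collision and showing client-only material effects.
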(event `InitColor`
  (switch `/Game/Data/E_PlayerColor` (select `int` (`KismetMathLibrary.RandomIntegerInRange` 0 7) :`0` "NewEnumerator0" :`1` "NewEnumerator1" :`2` "NewEnumerator2" :`3` "NewEnumerator3" :`4` "NewEnumerator4" :`5` "NewEnumerator5" :`6` "NewEnumerator6" :`7` "NewEnumerator7" :!type "/Game/Data/E_PlayerColor Enum")
    (:`NewEnumerator0`
      (set `self.animation_set` (`self.animation_set_Black`)))
    (:`NewEnumerator1`
      (set `self.animation_set` (`self.animation_set_Blue`)))
    (:`NewEnumerator2`
      (set `self.animation_set` (`self.animation_set_Green`)))
    (:`NewEnumerator3`
      (set `self.animation_set` (`self.animation_set_Pink`)))
    (:`NewEnumerator4`
      (set `self.animation_set` (`self.animation_set_Red`)))
    (:`NewEnumerator5`
      (set `self.animation_set` (`self.animation_set_Orange`)))
    (:`NewEnumerator6`
      (set `self.animation_set` (`self.animation_set_White`)))
    (:`NewEnumerator7`
      (set `self.animation_set` (`self.animation_set_Yellow`)))))

(event `ReturnSprite`
  (params (right :type Boolean))
  ;[0.1816 0.351 1] [ON EACH] Rotate FlipBook
  (`SceneComponent.K2_SetRelativeRotation` (`self.HeroFlipbook`) (select `bool` right :`false` (struct :`Yaw` 180.0) :!type "Rotator Structure") false false))

(event `CheckRotationFlipbook`
  (params (axis :type "Float (double-precision)"))
  ;[0.7682 0.4567 1] [SERVER] Check Rotation FlipBook
  (`/Engine/EditorBlueprintResources/StandardMacros.CompareFloat` axis
    (:`>`
      (`self.ReturnSprite` false))
    (:`<`
      (`self.ReturnSprite` true))))

(event `self.ReceiveAnyDamage`
  (params (Damage :type "Float (single-precision)") (DamageType :type "DamageType Object Reference") (InstigatedBy :type "Controller Object Reference") (DamageCauser :type "Actor Object Reference"))
  ;[0.7682 0.4567 1] [SERVER] Any Damage
  (if (not (`self.is_damaged`))
    (bind _backimpulse (`self.ComputeImpulseOrientation` DamageCauser))
    (`self.ManageDamage` _backimpulse)))

(event `DashAction`
  (params (Right :type Boolean))
  ;[0.7682 0.4567 1] [SERVER] Dash Call
  (`self.ApplyDash` Right))

(event `ApplyDamageOnClient`
  ;[0.1816 0.351 1] [ON EACH] Apply Damages / Update Client HUD
  (set `self.is_damaged` true))

(event `ApplyDash`
  (params (Right :type Boolean))
  (bind _dash_velocity (`self.dash_velocity`))
  ;[0.1816 0.351 1] [ON EACH] Apply Dash Movement
  (if (< (`self.dash_counter`) (`self.max_dash`))
    (`/Engine/EditorBlueprintResources/StandardMacros.IncrementInt` (`self.dash_counter`)
      (:`  `
        (`self.LaunchCharacter` (`KismetMathLibrary.MakeVector` (select `bool` Right :`false` (- 0.0 _dash_velocity) :`true` _dash_velocity) 0.0 100.0) true true)
        (`self.JumpFX`)))))

(event `self.ReceiveBeginPlay`
  (bind _heroflipbook (`self.HeroFlipbook`))
  ;[1 0.121 0.2007] Begin Play / OnPossessed Event
  (`KismetSystemLibrary.PrintString` "Hello")
  (`self.InitColor`)
  (bind _returnvalue (`PrimitiveComponent.CreateDynamicMaterialInstance` _heroflipbook 0 "/Game/Materials/M_Damaged.M_Damaged"))
  (set `self.dynamic_mat_ref` _returnvalue)
  (`PrimitiveComponent.SetMaterial` _heroflipbook 0 null))

(event `UpdateAnimation`
  (bind _returnvalue (`KismetMathLibrary.VSize` (`self.GetVelocity`)))
  ;[0.1816 0.351 1] [ON EACH] Update Movement On player State and Set Animation only for client
  (`|ExecutionSequence`
    (:`then_0`
      (set `self.is_moving` (> _returnvalue 0.0))
      (set `self.is_falling` (> _returnvalue 1450.0))
      (set `self.is_start_falling` (< (.z (`self.GetVelocity`)) 0.0))
      (set `self.is_jumping` (`NavMovementComponent.IsFalling` (`self.CharacterMovement`))))
    (:`then_1`
      (`self.AnimationStateMachine`))))

(event `ManageDamage`
  (params (BackImpulse :type Boolean))
  ;[0.3059 1 0.2732] Damage Manager / Apply damage / Launch Character / Check Dead
  (`self.ApplyDamageOnClient`)
  (`self.LaunchCharacter` (`KismetMathLibrary.GreaterGreater_VectorRotator` (`KismetMathLibrary.MakeVector` (* 400.0 (select `bool` BackImpulse :`false` 1.0 :`true` -1.0 :!type "Float (single-precision)")) 0.0 600.0) (`self.K2_GetActorRotation`)) true true)
  (`self.IsInvincible` true))

(event `self.ReceiveTick`
  (params (DeltaSeconds :type "Float (single-precision)"))
  ;[1 0.121 0.2007] Event Tick
  (`self.UpdateAnimation`))

(event `JumpAction`
  ;[0.7682 0.4567 1] [SERVER] Jump Call
  (`self.JumpManager`))

(event `self.OnLanded`
  (params (Hit :type "HitResult Structure (by ref)"))
  ;[1 0.121 0.2007] On Landed
  (set `self.jump_counter` 0)
  (set `self.dash_counter` 0))

(event `JumpManager`
  ;[0.1816 0.351 1] [ON EACH] Jump / MultiJump
  (if (< (`self.jump_counter`) (`self.max_jump`))
    (if (`self.CanJump`)
      (`self.Jump`)
      (else
        (`self.MultiJump`)))))

(event `MultiJump`
  (bind _returnvalue (`self.K2_GetActorLocation`))
  (bind _capsulecomponent (`self.CapsuleComponent`))
  (bind _returnvalue_2 (* (`SceneComponent.GetForwardVector` _capsulecomponent) (+ (`CapsuleComponent.GetScaledCapsuleRadius` _capsulecomponent) 40.0)))
  ;[0.1816 0.351 1] [ON EACH] Jump / MultiJump
  (`/Engine/EditorBlueprintResources/StandardMacros.IncrementInt` (`self.jump_counter`)
    (:`  `
      (bind (_outhit _returnvalue_3) (`KismetSystemLibrary.LineTraceSingle` :`Start` (- _returnvalue _returnvalue_2) :`End` (+ _returnvalue _returnvalue_2) :`TraceChannel` "TraceTypeQuery2" :`DrawTime` 0.0))
      (if _returnvalue_3
        (`self.WallJump` _outhit)
        (else
          (`self.Rejump`))))))

(event `IsInvincible`
  (params (invicible :type Boolean))
  ;[0.1816 0.351 1] [ON EACH] Is Invicible / Set Material and Collision Only on Clients
  (`|ExecutionSequence`
    (:`then_0`
      (`self.ChangeOverlap` invicible)
      (`/Engine/EditorBlueprintResources/ActorMacros.Switch Has Authority`
        (:`Remote`
          (`PrimitiveComponent.SetMaterial` (`self.HeroFlipbook`) 0 (select `bool` invicible :`true` (`self.dynamic_mat_ref`)))
          (`self.twinkle` invicible))))
    (:`then_1`
      (if invicible
        (`KismetSystemLibrary.Delay` 1.5)
        (set `self.is_damaged` false)
        (`/Engine/EditorBlueprintResources/ActorMacros.Switch Has Authority`
          (:`Authority`
            (`self.IsInvincible` false)))))))

(event `FireAction`
  ;[0.7682 0.4567 1] [SERVER] Fire Projectile
  (`self.Attack`)
  (`KismetSystemLibrary.Delay` 0.26)
  (bind _returnvalue (`|SpawnActorFromClass` "/Game/Blueprints/Characters/Hero/BP_StickMan_Projectile.BP_StickMan_Projectile_C" (`SceneComponent.K2_GetComponentToWorld` (`self.ProjectileSpawn`)) "AlwaysSpawn" "OverrideRootScale" null self))
  (`PrimitiveComponent.IgnoreActorWhenMoving` (`self.CapsuleComponent`) _returnvalue true))

(event `ChangeOverlap`
  (params (ignore :type Boolean))
  (bind _capsulecomponent (`self.CapsuleComponent`))
  ;[0.3059 1 0.2732] Change all channel overlap
  (`PrimitiveComponent.SetCollisionResponseToAllChannels` _capsulecomponent (select `bool` ignore :`false` "ECR_Block" :`true` "ECR_Ignore" :!type "ECollisionResponse Enum"))
  (`PrimitiveComponent.SetCollisionResponseToChannel` _capsulecomponent "ECC_Visibility" "ECR_Ignore")
  (`PrimitiveComponent.SetCollisionResponseToChannel` _capsulecomponent "ECC_WorldStatic" "ECR_Block"))

(event `Attack`
  ;[0.7682 0.4567 1] [SERVER] Fire Projectile
  (set `self.is_attacking` true)
  (`KismetSystemLibrary.Delay` (`PaperFlipbook.GetTotalDuration` (`BlueprintMapLibrary.Map_Find` (`self.animation_set`) "NewEnumerator4")))
  (set `self.is_attacking` false))

(event `twinkle`
  (params (activate :type Boolean))
  ;[0.3059 1 0.2732] Twinkle Effect
  (if activate
    (`Timeline|Timeline_0` :!via `PlayFromStart`
      (:`Update`
        (`MaterialInstanceDynamic.SetScalarParameterValue` (`self.dynamic_mat_ref`) "color" 0.0)))))

(event `WallJump`
  (params (hit :type "HitResult Structure"))
  (bind (_bblockinghit _binitialoverlap _time _location _impactpoint _normal _impactnormal _physmat _hitactor _hitcomponent _hitbonename _hititem _faceindex _tracestart) (`GameplayStatics.BreakHitResult` hit))
  (bind (_returnvalue_x _returnvalue_y) (`KismetMathLibrary.BreakVector` (`self.K2_GetActorLocation`)))
  ;[0.1816 0.351 1] [ON EACH] Wall Jump
  (`self.LaunchCharacter` (`KismetMathLibrary.MakeVector` (* (`KismetMathLibrary.SignOfFloat` (`KismetMathLibrary.Conv_IntToDouble` (`KismetMathLibrary.Round` (- _returnvalue_x (.x _location))))) (`self.jump_velocity`)) (* (`KismetMathLibrary.SignOfFloat` (`KismetMathLibrary.Conv_IntToDouble` (`KismetMathLibrary.Round` (- _returnvalue_y (.y _location))))) (`self.jump_velocity`)) (`self.jump_velocity`)) true true)
  (`self.JumpFX`)
  (`self.ReturnSprite` (not (== _impactpoint _tracestart))))

(event `Rejump`
  ;[0.1816 0.351 1] [ON EACH] Rejump
  (`self.LaunchCharacter` (`KismetMathLibrary.MakeVector` 0.0 0.0 (`self.jump_velocity`)) false true)
  (`self.JumpFX`))

(event `JumpFX`
  ;[0.3059 1 0.2732] [ON ECAH] Jump FX Only For Client
  (`/Engine/EditorBlueprintResources/ActorMacros.Switch Has Authority`
    (:`Remote`
      (`GameplayStatics.SpawnEmitterAtLocation` "/Game/Particles/pDust.pDust" (`SceneComponent.K2_GetComponentLocation` (`self.DustBox`)) (struct)))))

(fn `AnimationStateMachine`
  (locals (NewLocalVar_0 :type "/Game/Data/E_AnimationState Enum" :default "NewEnumerator0") (animation_tmp :type "/Game/Data/E_AnimationState Enum"))
  (set `local.animation_tmp` (`self.animation`))
  (if (`self.is_dashing`)
    (set `self.animation` "NewEnumerator3")
    (elif (`self.is_attacking`)
      (`KismetSystemLibrary.PrintString` "PAFFF")
      (set `self.animation` "NewEnumerator4")
      (elif (`self.is_damaged`)
        (set `self.animation` "NewEnumerator8")
        (elif (`self.is_falling`)
          (set `self.animation` "NewEnumerator5")
          (elif (`self.is_start_falling`)
            (set `self.animation` "NewEnumerator6")
            (elif (`self.is_jumping`)
              (set `self.animation` "NewEnumerator2")
              (elif (`self.is_moving`)
                (set `self.animation` "NewEnumerator1")
                (else
                  (set `self.animation` "NewEnumerator0")))))))))
  (if (`|EnumInequality` (`local.animation_tmp`) (`self.animation`))
    (`PaperFlipbookComponent.SetFlipbook` (`self.HeroFlipbook`) (`BlueprintMapLibrary.Map_Find` (`self.animation_set`) (`self.animation`)))))

(fn `ComputeImpulseOrientation`
  (params (DamageCauser :type "Actor Object Reference"))
  (returns (BackImpulse :type Boolean))
  (bind _returnvalue_x (`KismetMathLibrary.BreakVector` (- (`self.K2_GetActorLocation`) (`self.K2_GetActorLocation` DamageCauser))))
  (return (<= _returnvalue_x 0.0)))

(fn `UserConstructionScript`
  (bind _returnvalue_x (`KismetMathLibrary.BreakVector` (`self.GetActorScale3D`)))
  (set `CharacterMovementComponent.JumpZVelocity` (`self.jump_velocity`) (`self.CharacterMovement`))
  (set `self.JumpMaxHoldTime` 0.4)
  (set `self.current_scale` _returnvalue_x))