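; Player controller for the multiplayer Paper2D lobby, handling player profile, lobby UI and pawn input.
; Initial setup loads or creates the saved profile, then CallUpdate has the game mode swap the character and refresh everyone.
; Events fill the lobby widget with players and map settings or switch to a loading screen.
; Movement, fire, jump and dash forward to LobbyPawn; kicking opens MainMenu, and EndPlay destroys the session.
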(event `self.ReceiveBeginPlay`
  (`KismetSystemLibrary.PrintString` "Hello")
  (bind _aslobby_pawn (cast `/Game/Blueprints/Lobby/LobbyPawn` (`GameplayStatics.GetPlayerPawn` 0)))
  (set `self.player_ref` _aslobby_pawn))

(event `InputAxis|HonrizontalMove`
  (params (AxisValue :type "Float (single-precision)"))
  (bind _player_ref (`self.player_ref`))
  ;[0.7682 0.4567 1] [SERVER] All Input Call
  (`/Engine/EditorBlueprintResources/StandardMacros.IsValid` _player_ref
    (:`Is Valid`
      (`/Game/Blueprints/Lobby/LobbyPawn.CheckRotationFlipbook` _player_ref AxisValue)
      (`Pawn.AddMovementInput` _player_ref (`SceneComponent.GetForwardVector` (`Character.CapsuleComponent` _player_ref)) AxisValue false))))

(event `InitialSetup`
  (`self.SaveGameCheck`)
  (`self.CallUpdate` (`self.player_settings`)))

(event `UpdateAvailableCharacter`
  (params (availlableCharacter :type "Array of Boolean")))

(event `SetupLobbyMenu`
  (params (ServerName :type Text))
  (set `self.bShowMouseCursor` true)
  (bind _returnvalue (`|CreateWidget` "/Game/UI/Lobby/LobbyMenu.LobbyMenu_C" null ServerName))
  (bind _output_get (set `self.lobby_menu_HUD` _returnvalue))
  (`UserWidget.AddToViewport` _output_get 0)
  (`WidgetBlueprintLibrary.SetInputMode_GameAndUIEx` self _output_get))

(event `InputAction|fire`
  (params (Key :type "Key Structure" :default "AnyKey"))
  (bind _player_ref (`self.player_ref`))
  ;[0.7682 0.4567 1] [SERVER] All Input Call
  (:`Pressed`
    (`/Engine/EditorBlueprintResources/StandardMacros.IsValid` _player_ref
      (:`Is Valid`
        (`/Game/Blueprints/Lobby/LobbyPawn.FireAction` _player_ref)))))

(event `InputAction|Jump`
  (params (Key :type "Key Structure" :default "AnyKey"))
  (bind _player_ref (`self.player_ref`))
  ;[0.7682 0.4567 1] [SERVER] All Input Call
  (:`Pressed`
    (`/Engine/EditorBlueprintResources/StandardMacros.IsValid` _player_ref
      (:`Is Valid`
        (`/Game/Blueprints/Lobby/LobbyPawn.JumpAction` _player_ref))))
  (:`Released`
    (`Character.StopJumping` _player_ref)))

(event `InputAction|LeftDash`
  (params (Key :type "Key Structure" :default "AnyKey"))
  (bind _player_ref (`self.player_ref`))
  ;[0.7682 0.4567 1] [SERVER] All Input Call
  (:`Pressed`
    (`/Engine/EditorBlueprintResources/StandardMacros.IsValid` _player_ref
      (:`Is Valid`
        (`/Game/Blueprints/Lobby/LobbyPawn.DashAction` _player_ref false)))))

(event `CallUpdate`
  (params (player_infos :type "/Game/Blueprints/AllLevels/S_PlayerInfos Structure") (changed_status :type Boolean))
  (bind _aspaper_lobby_game_mode (cast `/Game/Blueprints/Lobby/PaperLobbyGameMode` (`GameplayStatics.GetGameMode`) :!pure true))
  (set `self.player_settings` player_infos)
  (`/Game/Blueprints/Lobby/PaperLobbyGameMode.SwapCharacter` _aspaper_lobby_game_mode self (`.player_character_16_D9E166954B22D792D35D8B8AE694F48A` (break `/Game/Blueprints/AllLevels/S_PlayerInfos` (`self.player_settings`))) changed_status)
  (`/Game/Blueprints/Lobby/PaperLobbyGameMode.EveryOneUpdate` _aspaper_lobby_game_mode))

(event `InputAction|RightDash`
  (params (Key :type "Key Structure" :default "AnyKey"))
  (bind _player_ref (`self.player_ref`))
  ;[0.7682 0.4567 1] [SERVER] All Input Call
  (:`Pressed`
    (`/Engine/EditorBlueprintResources/StandardMacros.IsValid` _player_ref
      (:`Is Valid`
        (`/Game/Blueprints/Lobby/LobbyPawn.DashAction` _player_ref true)))))

(event `AddPlayerInfos`
  (params (connectedPlayers :type "Array of /Game/Blueprints/AllLevels/S_PlayerInfos Structure"))
  (bind _lobby_menu_hud (`self.lobby_menu_HUD`))
  (set `self.AllConnectedPlayers` connectedPlayers)
  (`/Engine/EditorBlueprintResources/StandardMacros.IsValid` _lobby_menu_hud
    (:`Is Valid`
      (`/Game/UI/Lobby/LobbyMenu.ClearPlayerList` _lobby_menu_hud)
      (for _array_element (`self.AllConnectedPlayers`)
        (`/Game/UI/Lobby/LobbyMenu.UpdatePlayerWindow` (`self.lobby_menu_HUD`) _array_element)))))

(event `UpdateLobbySettings`
  (params (MapImage :type "Texture2D Object Reference") (MapName :type Text) (MapTime :type Text))
  (bind _lobby_menu_hud (`self.lobby_menu_HUD`))
  (set `/Game/UI/Lobby/LobbyMenu.map_image` MapImage _lobby_menu_hud)
  (set `/Game/UI/Lobby/LobbyMenu.map_name` MapName _lobby_menu_hud)
  (set `/Game/UI/Lobby/LobbyMenu.map_time` MapTime _lobby_menu_hud))

(event `ShowLoadingScreen`
  (`Widget.RemoveFromParent` (`self.lobby_menu_HUD`))
  (bind _returnvalue (`|CreateWidget` "/Game/UI/AllLevels/LoadingScreen.LoadingScreen_C" self))
  (`UserWidget.AddToViewport` _returnvalue 0))

(event `UpdatePlayersNumbers`
  (params (currentPlayers :type Integer) (maxPlayers :type Integer))
  (bind _lobby_menu_hud (`self.lobby_menu_HUD`))
  (`/Engine/EditorBlueprintResources/StandardMacros.IsValid` _lobby_menu_hud
    (:`Is Valid`
      (set `/Game/UI/Lobby/LobbyMenu.players_display` (`|FormatText` "{CurrentPlayers} of {MaxPlayers}" (`KismetTextLibrary.Conv_IntToText` currentPlayers) (`KismetTextLibrary.Conv_IntToText` maxPlayers)) _lobby_menu_hud))))

(event `self.ReceiveEndPlay`
  (params (EndPlayReason :type "EEndPlayReason Enum" :default "Destroyed"))
  (`DestroySessionCallbackProxy.DestroySession` self))

(event `Kicked`
  (`GameplayStatics.OpenLevel` "MainMenu"))

(fn `LoadGame`
  (bind _returnvalue (`GameplayStatics.LoadGameFromSlot` "player_settings_save"))
  (bind _aspaper_2dsaved_game (cast `/Game/Blueprints/AllLevels/Paper2DSavedGame` _returnvalue))
  (bind (_player_name _player_image) (break `/Game/Blueprints/AllLevels/S_PlayerInfos` (`/Game/Blueprints/AllLevels/Paper2DSavedGame.S_player_infos` _aspaper_2dsaved_game)))
  (setmembers `/Game/Blueprints/AllLevels/S_PlayerInfos` :`StructRef` (`self.player_settings`) :`player_name` _player_name :`player_image` _player_image :`player_character` "/Script/Paper2D.PaperCharacter" :`player_character_image` null :`player_status` "Not Ready"))

(fn `SaveGame`
  (bind _player_save_game_ref (`self.player_save_game_ref`))
  (`/Engine/EditorBlueprintResources/StandardMacros.IsValid` (`self.player_save_game_ref`)
    (:`Is Valid`
      _)
    (:`Is Not Valid`
      (bind _returnvalue (`GameplayStatics.CreateSaveGameObject` "/Game/Blueprints/AllLevels/Paper2DSavedGame.Paper2DSavedGame_C"))
      (set `self.player_save_game_ref` _returnvalue)))
  (set `/Game/Blueprints/AllLevels/Paper2DSavedGame.S_player_infos` (`self.player_settings`) _player_save_game_ref)
  (`GameplayStatics.SaveGameToSlot` _player_save_game_ref (`self.player_settings_save`)))

(fn `SaveGameCheck`
  (bind _returnvalue (`GameplayStatics.DoesSaveGameExist` (`self.player_settings_save`)))
  (if _returnvalue
    (`self.LoadGame`)
    (`self.SaveGame`)
    (else
      (`self.SaveGame`))))

(fn `UserConstructionScript`)