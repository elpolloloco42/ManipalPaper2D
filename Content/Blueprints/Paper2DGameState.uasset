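; Game state for a Paper2D game that holds the player list and spawns the level.
; On BeginPlay it spawns the Paper2D level Blueprint, calls its InitLevelActors and caches the first player controller.
; AddInfos appends player info, labelled as coming from the GameMode.
; AddInfos and SpawnLevel are labelled server-side, but the graph contains no authority check.
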(event `AddInfos`
  (params (infos :type "/Game/Data/S_OldPlayerInfos Structure"))
  ;[0.7682 0.4567 1] [SERVER] Add Infos From GameMode
  (`KismetArrayLibrary.Array_Add` (`self.players`) infos))

(event `self.ReceiveBeginPlay`
  ;[1 0.121 0.2007] Begin Play
  (`|ExecutionSequence`
    (:`then_0`
      (`self.SpawnLevel`))
    (:`then_1`
      (bind _aspaper_2dplayer_controller (cast `/Game/Blueprints/Gameplay/Paper2DPlayerController` (`GameplayStatics.GetPlayerController` 0)))
      (set `self.PlayerController` _aspaper_2dplayer_controller))))

(event `SpawnLevel`
  ;[0.7682 0.4567 1] [SERVER] SpawnLevel Actor
  (bind _returnvalue (`|SpawnActorFromClass` "/Game/Blueprints/Level/Paper2D_LevelBlueprint.Paper2D_LevelBlueprint_C" (`KismetMathLibrary.MakeTransform` (0.0 0.0 0.0)) "Undefined" "OverrideRootScale"))
  (bind _output_get (set `self.level_ref` _returnvalue))
  (`/Game/Blueprints/Level/Paper2D_LevelBlueprint.InitLevelActors` _output_get))

(fn `UserConstructionScript`)