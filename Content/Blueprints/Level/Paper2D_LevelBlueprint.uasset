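; Level Blueprint that builds the world map from placed rooms and links their doors.
; InitLevelActors gives each BP_Room an ID and groups it under a BP_World spawned per WorldId.
; InitDoorConnexion then pairs unlinked doors both ways, cycling round-robin from the next world and retrying until FindUnusedDoor returns a free one.
; Finally, it sets MapCreated on Paper2DGameMode.
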(event `InitLevelActors`
  ;[0.3059 1 0.2732] Create World Actor And Spawn Actor from Room
  (bind _outactors (`GameplayStatics.GetAllActorsOfClass` "/Game/Blueprints/Level/BP_Room.BP_Room_C"))
  (for (_array_element _array_index) _outactors
    (`self.InitWorldMap` _array_element _array_index))
  (`self.InitDoorConnexion`)
  (`self.CustomEvent_0`))

(event `CustomEvent_0`
  (bind _aspaper_2dgame_mode (cast `/Game/Blueprints/Gameplay/Paper2DGameMode` (`GameplayStatics.GetGameMode`)))
  (set `/Game/Blueprints/Gameplay/Paper2DGameMode.map_created` true _aspaper_2dgame_mode)
  (`KismetSystemLibrary.PrintString` "MAP CREATED" true true (struct :`G` 0.66 :`B` 1.0 :`A` 1.0) 20.0))

(event `InitWorldMap`
  (params (room :type "/Game/Blueprints/Level/BP_Room Object Reference") (id :type Integer))
  (bind _world_id (`/Game/Blueprints/Level/BP_Room.world_id` room))
  ;[0.3059 1 0.2732] Init World / Spawn World / Add Room in World
  (`|ExecutionSequence`
    (:`then_0`
      (set `/Game/Blueprints/Level/BP_Room.room_id` id room))
    (:`then_1`
      (bind _keys (`BlueprintMapLibrary.Map_Keys` (`self.world_map`)))
      (if (not (`KismetArrayLibrary.Array_Contains` _keys _world_id))
        (bind _returnvalue (`|SpawnActorFromClass` "/Game/Blueprints/Level/BP_World.BP_World_C" (`KismetMathLibrary.MakeTransform` (0.0 0.0 0.0)) "Undefined" "OverrideRootScale" null _world_id))
        (`BlueprintMapLibrary.Map_Add` (`self.world_map`) _world_id _returnvalue)))
    (:`then_2`
      (`/Game/Blueprints/Level/BP_World.AddRoom` (`BlueprintMapLibrary.Map_Find` (`self.world_map`) (`/Game/Blueprints/Level/BP_Room.world_id` room)) room))))

(fn `FindUnusedDoor`
  (params (World :type "/Game/Blueprints/Level/BP_World Object Reference"))
  (returns (door_found :type Boolean) (door :type "/Game/Blueprints/Level/BP_Door Object Reference"))
  (locals (found :type Boolean))
  (bind _values (`BlueprintMapLibrary.Map_Values` (`/Game/Blueprints/Level/BP_World.room_list` World)))
  (for _array_element _values
    (for _array_element_2 (`/Game/Blueprints/Level/BP_Room.door_list` _array_element)
      (`/Engine/EditorBlueprintResources/StandardMacros.IsValid` (`/Game/Blueprints/Level/BP_Door.next_door_ref` _array_element_2)
        (:`Is Not Valid`
          (set `local.found` true)
          (break))))
    (if (`local.found`)
      (break)))
  (return (`local.found`) _array_element_2))

(fn `InitDoorConnexion`
  (locals (world_counter :type Integer) (world_id_tmp :type Integer))
  (bind _world_map (`self.world_map`))
  (set `local.world_counter` (`BlueprintMapLibrary.Map_Length` _world_map))
  (bind _values (`BlueprintMapLibrary.Map_Values` _world_map))
  (for _array_element _values
    (bind _output_get (set `local.world_id_tmp` (`/Game/Blueprints/Level/BP_World.id` _array_element)))
    (`/Engine/EditorBlueprintResources/StandardMacros.IncrementInt` _output_get
      (:`  `
        (bind _values_2 (`BlueprintMapLibrary.Map_Values` (`/Game/Blueprints/Level/BP_World.room_list` _array_element)))
        (for _array_element_2 _values_2
          (for _array_element_3 (`/Game/Blueprints/Level/BP_Room.door_list` _array_element_2)
            (`/Engine/EditorBlueprintResources/StandardMacros.IsValid` (`/Game/Blueprints/Level/BP_Door.next_door_ref` _array_element_3)
              (:`Is Not Valid`
                (bind (_door_found _door) (`self.FindUnusedDoor` (`BlueprintMapLibrary.Map_Find` (`self.world_map`) (mod (`local.world_id_tmp`) (`local.world_counter`))) :!label _label))
                (`/Engine/EditorBlueprintResources/StandardMacros.IncrementInt` (`local.world_id_tmp`)
                  (:`  `
                    (if _door_found
                      (set `/Game/Blueprints/Level/BP_Door.next_door_ref` _door _array_element_3)
                      (set `/Game/Blueprints/Level/BP_Door.next_door_ref` _array_element_3 _door)
                      (else
                        (goto _label)))))))))))))

(fn `UserConstructionScript`)