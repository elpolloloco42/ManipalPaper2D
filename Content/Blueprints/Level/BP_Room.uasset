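; BP_Room is a 2D room actor that displays an assigned Paper2D tile map as part of the level.
; The construction script applies the map, then sizes and centers a trigger box over it using its bounds and tile dimensions.
; On BeginPlay, tile map collision is enabled only if the room's WorldId matches the game state's current room.
; Hero overlap re-enables collision for the current room, while end overlap does nothing beyond a cast.
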(event `self.ReceiveBeginPlay`
  (`|ExecutionSequence`
    (:`then_0`
      (bind _aspaper_2dgame_state_base (cast `/Game/Blueprints/Paper2DGameStateBase` (`GameplayStatics.GetGameState`)))
      (set `self.game_state_ref` _aspaper_2dgame_state_base)
      (set `self.vertical_offset` 20.0))
    (:`then_2`
      (`PrimitiveComponent.SetCollisionEnabled` (`self.PaperTileMap`) (select `bool` (== (`self.world_id`) (`.world_id_17_3D1E126D45B5D38C34754FBFA4E87736` (break `/Game/Data/S_Room` (`/Game/Blueprints/Paper2DGameStateBase.current_room` (`self.game_state_ref`))))) :`false` "NoCollision" :`true` "QueryAndPhysics" :!type "ECollisionEnabled Enum")))))

(event `self.Collision.OnComponentBeginOverlap`
  (params (OverlappedComponent :type "PrimitiveComponent Object Reference") (OtherActor :type "Actor Object Reference") (OtherComp :type "PrimitiveComponent Object Reference") (OtherBodyIndex :type Integer) (bFromSweep :type Boolean) (SweepResult :type "HitResult Structure (by ref)"))
  (bind _game_state_ref (`self.game_state_ref`))
  (cast `/Game/Blueprints/Hero/Paper2DHero` OtherActor)
  (`/Engine/EditorBlueprintResources/StandardMacros.IsValid` _game_state_ref
    (:`Is Valid`
      (if (== (`self.world_id`) (`.world_id_17_3D1E126D45B5D38C34754FBFA4E87736` (break `/Game/Data/S_Room` (`/Game/Blueprints/Paper2DGameStateBase.current_room` _game_state_ref))))
        (`PrimitiveComponent.SetCollisionEnabled` (`self.PaperTileMap`) "QueryAndPhysics")))))

(event `self.Collision.OnComponentEndOverlap`
  (params (OverlappedComponent :type "PrimitiveComponent Object Reference") (OtherActor :type "Actor Object Reference") (OtherComp :type "PrimitiveComponent Object Reference") (OtherBodyIndex :type Integer))
  (cast `/Game/Blueprints/Hero/Paper2DHero` OtherActor))

(fn `UserConstructionScript`
  (locals (width_counter :type Integer) (height_counter :type Integer) (x :type Integer) (y :type Integer))
  (bind _collision (`self.Collision`))
  (bind _tile_length (`self.tile_length`))
  (bind _returnvalue (/ _tile_length 2))
  (`|ExecutionSequence`
    (:`then_0`
      (`PaperTileMapComponent.SetTileMap` (`self.PaperTileMap`) (`self.map`))
      (bind (_mapwidth _mapheight) (`PaperTileMapComponent.GetMapSize` (`self.PaperTileMap`)))
      (set `self.map_width` _mapwidth)
      (set `self.map_height` _mapheight))
    (:`then_1`
      (`BoxComponent.SetBoxExtent` _collision (`.BoxExtent` (`KismetSystemLibrary.GetComponentBounds` (`self.PaperTileMap`))) true)
      (`SceneComponent.K2_SetRelativeRotation` _collision (`SceneComponent.K2_GetComponentRotation` (`self.PaperTileMap`)) false false)
      (`SceneComponent.K2_AddRelativeLocation` _collision (`KismetMathLibrary.MakeVector` (`KismetMathLibrary.Conv_IntToDouble` (- (/ (* _tile_length (`self.map_width`)) 2) _returnvalue)) 0.0 (`KismetMathLibrary.Conv_IntToDouble` (- 0 (- (/ (* _tile_length (`self.map_height`)) 2) _returnvalue)))) false false))))