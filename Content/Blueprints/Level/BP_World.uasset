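; BP_World is a level Blueprint asset that acts as a registry of rooms, stored in a map keyed by RoomId.
; AddRoom hands each room a reference to the world, initializes it, adopts its Spawn if valid, then adds it to RoomList.
; SetWorldVisible loops over all rooms but does nothing, as its HideRoom call is disconnected and its Actor input is unused.
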(event `AddRoom`
  (params (room :type "/Game/Blueprints/Level/BP_Room Object Reference"))
  (bind _spawn (`/Game/Blueprints/Level/BP_Room.spawn` room))
  ;[0.3059 1 0.2732] Add Room to list / Init Room for Each
  (`|ExecutionSequence`
    (:`then_0`
      (set `/Game/Blueprints/Level/BP_Room.world` self room))
    (:`then_1`
      (`/Game/Blueprints/Level/BP_Room.InitRoom` room)
      (`/Engine/EditorBlueprintResources/StandardMacros.IsValid` _spawn
        (:`Is Valid`
          (set `self.spawn` _spawn))))
    (:`then_2`
      (`BlueprintMapLibrary.Map_Add` (`self.room_list`) (`/Game/Blueprints/Level/BP_Room.room_id` room) room))))

(fn `SetWorldVisible`
  (params (visible :type Boolean) (actor :type Boolean))
  (bind _values (`BlueprintMapLibrary.Map_Values` (`self.room_list`)))
  (for _array_element _values
    _))

(fn `UserConstructionScript`)