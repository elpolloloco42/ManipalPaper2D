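; BP_Ladder is a climbable ladder for the Paper2D hero, sized by its top and bottom points.
; The construction script spawns non-colliding rung sprites, stretches the climb box over the height and places an ejection box at the top.
; The climb box toggles OnLadder on the hero's controller, calling ClimbingEnd on exit.
; Touching the ejection box teleports the hero above it, then makes it block pawns, with no reset here.
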(event `self.Box.OnComponentBeginOverlap`
  (params (OverlappedComponent :type "PrimitiveComponent Object Reference") (OtherActor :type "Actor Object Reference") (OtherComp :type "PrimitiveComponent Object Reference") (OtherBodyIndex :type Integer) (bFromSweep :type Boolean) (SweepResult :type "HitResult Structure (by ref)"))
  (bind _aspaper_2dhero (cast `/Game/Blueprints/Hero/Paper2DHero` OtherActor))
  (set `/Game/Blueprints/Paper2DController.on_ladder` true (`/Game/Blueprints/Hero/Paper2DHero.player_controller_ref` _aspaper_2dhero)))

(event `self.Box.OnComponentEndOverlap`
  (params (OverlappedComponent :type "PrimitiveComponent Object Reference") (OtherActor :type "Actor Object Reference") (OtherComp :type "PrimitiveComponent Object Reference") (OtherBodyIndex :type Integer))
  (bind _aspaper_2dhero (cast `/Game/Blueprints/Hero/Paper2DHero` OtherActor))
  (bind _player_controller_ref (`/Game/Blueprints/Hero/Paper2DHero.player_controller_ref` _aspaper_2dhero))
  (set `/Game/Blueprints/Paper2DController.on_ladder` false _player_controller_ref)
  (`/Game/Blueprints/Paper2DController.ClimbingEnd` _player_controller_ref)
  (`KismetSystemLibrary.PrintString` "[END]"))

(event `self.EjectionBox.OnComponentBeginOverlap`
  (params (OverlappedComponent :type "PrimitiveComponent Object Reference") (OtherActor :type "Actor Object Reference") (OtherComp :type "PrimitiveComponent Object Reference") (OtherBodyIndex :type Integer) (bFromSweep :type Boolean) (SweepResult :type "HitResult Structure (by ref)"))
  (bind _ejectionbox (`self.EjectionBox`))
  (bind (_returnvalue_x _returnvalue_y _returnvalue_z) (`KismetMathLibrary.BreakVector` (`SceneComponent.K2_GetComponentLocation` _ejectionbox)))
  (bind _aspaper_2dhero (cast `/Game/Blueprints/Hero/Paper2DHero` OtherActor))
  (bind _capsulecomponent (`Character.CapsuleComponent` _aspaper_2dhero))
  (bind (_returnvalue_x_2 _returnvalue_y_2) (`KismetMathLibrary.BreakVector` (`SceneComponent.K2_GetComponentLocation` _capsulecomponent)))
  (`SceneComponent.K2_SetWorldLocation` _capsulecomponent (`KismetMathLibrary.MakeVector` _returnvalue_x_2 _returnvalue_y_2 (+ (.z (`.BoxExtent` (`KismetSystemLibrary.GetComponentBounds` _capsulecomponent))) _returnvalue_z (* 3 (.z (`.BoxExtent` (`KismetSystemLibrary.GetComponentBounds` _ejectionbox)))))) false false)
  (`PrimitiveComponent.SetCollisionResponseToChannel` (`self.EjectionBox`) "ECC_Pawn" "ECR_Block")
  (`KismetSystemLibrary.PrintString` "Hello"))

(fn `UserConstructionScript`
  (bind _rung_offset (`self.rung_offset`))
  (bind _box (`self.Box`))
  (bind (_ladder_top_x _ladder_top_y _ladder_top_z) (`KismetMathLibrary.BreakVector` (`self.ladder_top`)))
  (bind (_returnvalue_x _returnvalue_y _returnvalue_z) (`KismetMathLibrary.BreakVector` (- (`self.ladder_top`) (`self.ladder_bottom`))))
  (bind _returnvalue (/ _returnvalue_z 2.0))
  (`|ExecutionSequence`
    (:`then_0`
      (for _index (range (+ (`KismetMathLibrary.FTrunc` (/ _returnvalue_z _rung_offset)) 1))
        (bind _returnvalue_2 (`AddComponent|NODE_AddPaperSpriteComponent-0` :`RelativeTransform` (`KismetMathLibrary.MakeTransform` (`KismetMathLibrary.MakeVector` 0.0 0.0 (* _index _rung_offset)) (struct) (1.3 1.5 0.15))))
        (`PaperSpriteComponent.SetSprite` _returnvalue_2 (`self.ladder_sprite`))
        (`PrimitiveComponent.SetCollisionEnabled` _returnvalue_2 "NoCollision"))
      (`SceneComponent.SetRelativeScale3D` _box (`KismetMathLibrary.MakeVector` 1.0 1.0 _returnvalue))
      (`SceneComponent.K2_AddRelativeLocation` _box (`KismetMathLibrary.MakeVector` 0.0 0.0 _returnvalue) false false))
    (:`then_1`
      (`SceneComponent.K2_AddLocalOffset` (`self.EjectionBox`) (`KismetMathLibrary.MakeVector` _ladder_top_x _ladder_top_y (+ _ladder_top_z (.z (`.BoxExtent` (`KismetSystemLibrary.GetComponentBounds` (`self.EjectionBox`)))))) false false))))