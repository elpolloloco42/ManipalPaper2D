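; BP_Door is a level door for a 2D game that registers itself with the player controller while the hero stands in it.
; The construction script applies the DoorSprite variable to its sprite, and BeginPlay caches the Paper2DController.
; Box overlap with a Paper2DHero sets the controller's CurrentDoor and OnDoor flag.
; End overlap clears only the flag, leaving CurrentDoor set.
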(event `self.ReceiveBeginPlay`
  (bind _aspaper_2dcontroller (cast `/Game/Blueprints/Paper2DController` (`GameplayStatics.GetPlayerController` 0)))
  (set `self.player_controller_ref` _aspaper_2dcontroller))

(event `self.Box.OnComponentBeginOverlap`
  (params (OverlappedComponent :type "PrimitiveComponent Object Reference") (OtherActor :type "Actor Object Reference") (OtherComp :type "PrimitiveComponent Object Reference") (OtherBodyIndex :type Integer) (bFromSweep :type Boolean) (SweepResult :type "HitResult Structure (by ref)"))
  (bind _player_controller_ref (`self.player_controller_ref`))
  (cast `/Game/Blueprints/Hero/Paper2DHero` OtherActor)
  (set `/Game/Blueprints/Paper2DController.current_door` self _player_controller_ref)
  (set `/Game/Blueprints/Paper2DController.on_door` true _player_controller_ref))

(event `self.Box.OnComponentEndOverlap`
  (params (OverlappedComponent :type "PrimitiveComponent Object Reference") (OtherActor :type "Actor Object Reference") (OtherComp :type "PrimitiveComponent Object Reference") (OtherBodyIndex :type Integer))
  (cast `/Game/Blueprints/Hero/Paper2DHero` OtherActor)
  (set `/Game/Blueprints/Paper2DController.on_door` false (`self.player_controller_ref`)))

(fn `UserConstructionScript`
  (locals (sprite_size :type "Float (double-precision)" :default 206.0))
  (`PaperSpriteComponent.SetSprite` (`self.Sprite`) (`self.door_sprite`)))