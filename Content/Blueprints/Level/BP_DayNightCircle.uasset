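; BP_DayNightCircle drives a day-night cycle by rotating a Sun actor and refreshing a Sky actor.
; On BeginPlay it converts the day length in minutes into seconds per in-game hour.
; Each Tick advances the hour counter without wrapping it, maps it to a sun pitch, applies the rotation, then calls UpdateSunDirection on the sky.
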(event `self.ReceiveBeginPlay`
  (bind _output_get (set `self.one_day` (* (`self.day_lenght`) 60.0)))
  (set `self.one_hour` (/ _output_get 24.0)))

(event `self.ReceiveTick`
  (params (DeltaSeconds :type "Float (single-precision)"))
  (bind _output_get (set `self.Hour` (+ (/ DeltaSeconds (`self.one_hour`)) (`self.Hour`))))
  (bind _output_get_2 (set `self.sun_angle` (+ (* (/ _output_get 6.0) 90.0) 90.0)))
  (`self.K2_SetActorRotation` (`self.sun`) (`KismetMathLibrary.MakeRotator` 0.0 _output_get_2) false)
  (`/Engine/EngineSky/BP_Sky_Sphere.UpdateSunDirection` (`self.Sky`)))

(fn `UserConstructionScript`)