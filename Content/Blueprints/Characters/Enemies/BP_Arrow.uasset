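; BP_Arrow is an enemy arrow projectile that damages a Paper2DHero on hit and destroys itself.
; On any other hit it disables collision, then branches on network authority.
; The authority destroys the arrow after a short delay, while remote copies play a Wobble timeline that rotates the Scene component to show the impact.
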(event `self.ReceiveHit`
  (params (MyComp :type "PrimitiveComponent Object Reference") (Other :type "Actor Object Reference") (OtherComp :type "PrimitiveComponent Object Reference") (bSelfMoved :type Boolean) (HitLocation :type "Vector Structure") (HitNormal :type "Vector Structure") (NormalImpulse :type "Vector Structure") (Hit :type "HitResult Structure (by ref)"))
  ;[1 0.1412 0.2039] On Hit Event
  (bind _aspaper_2dhero (cast `/Game/Blueprints/Characters/Hero/Paper2DHero` Other)
    (:`then`
      (`GameplayStatics.ApplyDamage` _aspaper_2dhero 1.0 null self)
      (`self.K2_DestroyActor`))
    (:`CastFailed`
      (`PrimitiveComponent.SetCollisionEnabled` (`self.Collision`) "NoCollision")
      (`/Engine/EditorBlueprintResources/ActorMacros.Switch Has Authority`
        (:`Authority`
          (`KismetSystemLibrary.Delay` 2.0)
          (`self.K2_DestroyActor`))
        (:`Remote`
          (bind (_direction _wobble) (`Timeline|Wobble` :!via `PlayFromStart`)
            (:`Update`
              (`SceneComponent.K2_SetRelativeRotation` (`self.Scene`) (`KismetMathLibrary.RLerp` (struct) (struct :`Pitch` 100.0) _wobble) false false))))))))

(fn `UserConstructionScript`)