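; Base 2D Paper enemy that deals contact damage to the player and dies on any hit, dropping pickups.
; When damaged, it rolls against SpecialItemPop to spawn either rings or a random health or mushroom pickup, then destroys itself.
; The construction script fits the damage box to the flipbook bounds.
; ActivateEnemie toggles visibility and collision, though its only call in this graph is unconnected.
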(event `self.ReceiveBeginPlay`
  ;[1 0.1412 0.2039] BeginPlay
  (bind _aspaper_2dgame_state (cast `/Game/Blueprints/Paper2DGameState` (`GameplayStatics.GetGameState`)))
  (set `self.game_state_ref` _aspaper_2dgame_state))

(event `self.ReceiveAnyDamage`
  (params (Damage :type "Float (single-precision)") (DamageType :type "DamageType Object Reference") (InstigatedBy :type "Controller Object Reference") (DamageCauser :type "Actor Object Reference"))
  (bind _returnvalue (`KismetMathLibrary.RandomFloatInRange` 0.0 100.0))
  ;[0.7682 0.4567 1] [SERVER] Set Random Values / Spawn Items
  (`KismetSystemLibrary.PrintString` "DAMAGE ON ENEMY")
  (set `self.random_item_pop` _returnvalue)
  (set `self.random_ring_dropped` (`KismetMathLibrary.FTrunc` (/ _returnvalue 20.0)))
  (`self.SpawnItem`))

(event `self.Box.OnComponentBeginOverlap`
  (params (OverlappedComponent :type "PrimitiveComponent Object Reference") (OtherActor :type "Actor Object Reference") (OtherComp :type "PrimitiveComponent Object Reference") (OtherBodyIndex :type Integer) (bFromSweep :type Boolean) (SweepResult :type "HitResult Structure (by ref)"))
  ;[1 0.1412 0.2039] Overlap player and damage him
  (bind _aspaper_2dhero_base (cast `/Game/Blueprints/Characters/Hero/Paper2DHeroBase` OtherActor))
  (`GameplayStatics.ApplyDamage` _aspaper_2dhero_base 1.0 null self))

(event `SpawnItem`
  (bind (_returnvalue_location _returnvalue_rotation) (`KismetMathLibrary.BreakTransform` (`self.GetTransform`)))
  ;[0.3059 1 0.2732] Death and drop random item
  (`/Engine/EditorBlueprintResources/StandardMacros.CompareFloat` (`self.random_item_pop`) (`self.special_item_pop`)
    (:`>`
      (for _ (range (+ (`self.random_ring_dropped`) 1)) :!label _label
        (`|SpawnActorFromClass` "/Game/Blueprints/PickUp/BP_PickUp_Ring.BP_PickUp_Ring_C" (`KismetMathLibrary.MakeTransform` _returnvalue_location _returnvalue_rotation) "AlwaysSpawn" "OverrideRootScale")))
    (:`==`
      (goto _label))
    (:`<`
      (`|SpawnActorFromClass` (select `bool` (`KismetMathLibrary.RandomBool`) :`false` "/Game/Blueprints/PickUp/BP_PickUpMushroom.BP_PickUpMushroom_C" :`true` "/Game/Blueprints/PickUp/BP_PickUp_Health.BP_PickUp_Health_C" :!type "/Game/Blueprints/PickUp/BP_PickUpBase Class Reference") (`KismetMathLibrary.MakeTransform` _returnvalue_location _returnvalue_rotation) "Undefined" "OverrideRootScale")))
  (`self.K2_DestroyActor`))

(fn `ActivateEnemie`
  (params (Active :type Boolean))
  (bind _output_get (set `self.active` Active))
  (`self.SetActorHiddenInGame` (not _output_get))
  (`self.SetActorEnableCollision` Active))

(fn `UserConstructionScript`
  (bind (_returnvalue_x _returnvalue_y _returnvalue_z) (`KismetMathLibrary.BreakVector` (`KismetMathLibrary.TransformDirection` (`KismetMathLibrary.MakeTransform` (0.0 0.0 0.0) (`self.K2_GetActorRotation`)) (`.BoxExtent` (`KismetSystemLibrary.GetComponentBounds` (`self.PaperFlipbook`))))))
  ;[0.3325 0.162 0.3864] Set collision scale to sprite scale
  (`BoxComponent.SetBoxExtent` (`self.Box`) (`KismetMathLibrary.MakeVector` (`KismetMathLibrary.Abs` _returnvalue_x) 50.0 (+ (`KismetMathLibrary.Abs` _returnvalue_z) (`self.delta`))) true))