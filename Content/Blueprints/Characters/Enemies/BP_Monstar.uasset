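; BP_Monstar is a Paper2D enemy with a walk flipbook that moves between its construction-time location and an EndLocation.
; On BeginPlay, AttackMovement, marked as server-side, plays a timeline that lerps the actor's location without sweeping.
; Each update also calls UpdateRotation, which on non-authority instances mirrors the sprite's X scale near the path ends, using paired DoOnce gates to avoid repeated flips.
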(event `self.ReceiveBeginPlay`
  ;[1 0.121 0.2007] Begin Play
  (`self.AttackMovement`))

(event `AttackMovement`
  ;[0.7682 0.4567 1] [SERVER] Attack Movement
  (bind (_direction _delta) (`Timeline|timeline_monstar_movement` :`NewTime` 2.0)
    (:`Update`
      (`self.K2_SetActorLocation` (`KismetMathLibrary.VLerp` (`self.start_location`) (`self.end_location`) _delta))
      (`self.UpdateRotation` _delta))))

(event `UpdateRotation`
  (params (delta :type "Float (double-precision)"))
  (bind _paperflipbook (`self.PaperFlipbook`))
  ;[0.1816 0.351 1] [ON EACH] Update Rotation Only on Client
  (`/Engine/EditorBlueprintResources/ActorMacros.Switch Has Authority`
    (:`Remote`
      (if (<= delta 0.01)
        (`|ExecutionSequence`
          (:`then_0`
            (`/Engine/EditorBlueprintResources/StandardMacros.DoOnce` false :!label _label
              (:`Completed`
                (`SceneComponent.SetWorldScale3D` _paperflipbook (-1.0 1.0 1.0)))))
          (:`then_1`
            (goto _label_2 :!via `Reset`)))
        (elif (>= delta 0.99)
          (`|ExecutionSequence`
            (:`then_0`
              (`/Engine/EditorBlueprintResources/StandardMacros.DoOnce` false :!label _label_2
                (:`Completed`
                  (`SceneComponent.SetWorldScale3D` _paperflipbook (1.0 1.0 1.0)))))
            (:`then_1`
              (goto _label :!via `Reset`))))))))

(fn `UserConstructionScript`
  (`PaperFlipbookComponent.SetFlipbook` (`self.PaperFlipbook`) "/Game/Animations/monstar_walk.monstar_walk")
  (set `self.start_location` (`self.K2_GetActorLocation`))
  (set `self.delta` 0.0)
  (`parent.UserConstructionScript`))