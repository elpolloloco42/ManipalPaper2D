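; Arrow trap enemy that fires a BP_Arrow from its SpawnPoint on a looping timer while a timeline moves it.
; At BeginPlay it sets its yaw from the Orientation setting, records its start position and starts the fire timer.
; The construction script derives a movement vector from SpawnPoint rotation, Orientation and Speed, which acts as travel distance for the timeline's location lerp.
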(event `Fire`
  (bind (_returnvalue_location _returnvalue_rotation _returnvalue_scale) (`KismetMathLibrary.BreakTransform` (`SceneComponent.K2_GetComponentToWorld` (`self.SpawnPoint`))))
  ;[0.3059 1 0.2732] Fire
  (`|SpawnActorFromClass` "/Game/Blueprints/Characters/Enemies/BP_Arrow.BP_Arrow_C" (`KismetMathLibrary.MakeTransform` (+ _returnvalue_location (0.0 -0.1 0.0)) _returnvalue_rotation _returnvalue_scale) "Undefined" "OverrideRootScale"))

(event `self.ReceiveBeginPlay`
  ;[1 0.1216 0.1725] Event begin play
  (`self.InitTrap`)
  (`self.AttackMovement`))

(event `InitTrap`
  ;[0.7682 0.4567 1] [SERVER] Init Trap Rotation / Launch Attack
  (`self.K2_SetActorRelativeRotation` (select `/Game/Data/E_Orientation` (`self.orientation`) :`NewEnumerator0` (struct :`Pitch` 90.0) :`NewEnumerator1` (struct :`Pitch` 270.0) :`NewEnumerator3` (struct :`Pitch` 180.0) :!type "Rotator Structure"))
  (set `self.start_position` (`self.K2_GetActorLocation`))
  (bind _returnvalue (`KismetSystemLibrary.K2_SetTimer` null "Fire" 1.5 true))
  (set `self.arrow_timer` _returnvalue))

(event `AttackMovement`
  (bind _start_position (`self.start_position`))
  ;[0.7682 0.4567 1] [SERVER] Attack Movement
  (bind (_direction _movement) (`Timeline|Timeline_Trap_Movement`)
    (:`Update`
      (`self.K2_SetActorLocation` (`KismetMathLibrary.VLerp` _start_position (+ _start_position (`self.movement_vector`)) _movement)))))

(fn `UserConstructionScript`
  (bind _speed (`self.speed`))
  (bind _returnvalue (`KismetMathLibrary.MakeVector` 0.0 0.0 _speed))
  (bind _returnvalue_2 (`KismetMathLibrary.MakeVector` _speed))
  (bind (_returnvalue_location _returnvalue_rotation) (`KismetMathLibrary.BreakTransform` (`SceneComponent.K2_GetComponentToWorld` (`self.SpawnPoint`))))
  (set `self.movement_vector` (`KismetMathLibrary.TransformDirection` (`KismetMathLibrary.MakeTransform` (0.0 0.0 0.0) _returnvalue_rotation) (select `/Game/Data/E_Orientation` (`self.orientation`) :`NewEnumerator0` _returnvalue_2 :`NewEnumerator1` _returnvalue_2 :`NewEnumerator2` _returnvalue :`NewEnumerator3` _returnvalue))))