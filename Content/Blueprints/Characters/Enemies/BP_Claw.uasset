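; BP_Claw is a networked Paper2D enemy that starts lowered and rises to its placed position to attack nearby heroes.
; Server-side DetectionBox overlaps call Attack, whose timeline lerps the claw between both positions, repeating while Attack is true.
; On clients, paired DoOnce gates toggle flipbook visibility as the timeline crosses its midpoint.
; The SpawnItem override drops rings or a health/mushroom pickup at the placed position, then destroys the actor.
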(event `Attack`
  (params (attack :type Boolean))
  ;[0.7682 0.4567 1] [SERVER] Attack Movement
  (bind (_direction _delta) (`Timeline|timeline_claw_movement` :!label _label)
    (:`Update`
      (`self.K2_SetActorLocation` (`KismetMathLibrary.VLerp` (`self.start_location`) (`self.end_location`) _delta))
      (`self.UpdateVisibility` _delta))
    (:`Finished`
      (if attack
        (goto _label :!via `PlayFromStart`)
        (else
          (goto _label :!via `Stop`))))))

(event `self.ReceiveBeginPlay`
  ;[1 0.1235 0.1732] Begin play
  (`self.K2_SetActorLocation` (`self.start_location`))
  (`/Engine/EditorBlueprintResources/ActorMacros.Switch Has Authority`
    (:`Remote`
      (`SceneComponent.SetVisibility` (`self.PaperFlipbook`) false false))))

(event `self.DetectionBox.OnComponentBeginOverlap`
  (params (OverlappedComponent :type "PrimitiveComponent Object Reference") (OtherActor :type "Actor Object Reference") (OtherComp :type "PrimitiveComponent Object Reference") (OtherBodyIndex :type Integer) (bFromSweep :type Boolean) (SweepResult :type "HitResult Structure (by ref)"))
  ;[1 0.1216 0.1725] Overlap
  (cast `/Game/Blueprints/Characters/Hero/Paper2DHeroBase` OtherActor)
  (`/Engine/EditorBlueprintResources/ActorMacros.Switch Has Authority`
    (:`Authority`
      (`self.Attack` true))))

(event `UpdateVisibility`
  (params (delta :type "Float (double-precision)"))
  (bind _paperflipbook (`self.PaperFlipbook`))
  ;[0.1816 0.351 1] [ON EACH] UpdateVisibility Only on Client
  (`/Engine/EditorBlueprintResources/ActorMacros.Switch Has Authority`
    (:`Remote`
      (`/Engine/EditorBlueprintResources/StandardMacros.CompareFloat` delta 0.5
        (:`>`
          (`/Engine/EditorBlueprintResources/StandardMacros.DoOnce` false :!label _label_2
            (:`Completed`
              (`SceneComponent.SetVisibility` _paperflipbook true false)
              (goto _label_3 :!via `Reset`))))
        (:`<`
          (`/Engine/EditorBlueprintResources/StandardMacros.DoOnce` false :!label _label_3
            (:`Completed`
              (`SceneComponent.SetVisibility` _paperflipbook false false)
              (goto _label_2 :!via `Reset`))))))))

(event `self.DetectionBox.OnComponentEndOverlap`
  (params (OverlappedComponent :type "PrimitiveComponent Object Reference") (OtherActor :type "Actor Object Reference") (OtherComp :type "PrimitiveComponent Object Reference") (OtherBodyIndex :type Integer))
  ;[1 0.1216 0.1725] Overlap
  (cast `/Game/Blueprints/Characters/Hero/Paper2DHeroBase` OtherActor)
  (`/Engine/EditorBlueprintResources/ActorMacros.Switch Has Authority`
    (:`Authority`
      (`self.Attack` false))))

(event `self.SpawnItem`
  (bind _returnvalue (`self.K2_GetActorRotation`))
  (bind _end_location (`self.end_location`))
  ;[0.3059 1 0.2732] Override Drop Item
  (`/Engine/EditorBlueprintResources/StandardMacros.CompareFloat` (`self.random_item_pop`) (`self.special_item_pop`)
    (:`>`
      (for _ (range (+ (`self.random_ring_dropped`) 1)) :!label _label_4
        (`|SpawnActorFromClass` "/Game/Blueprints/PickUp/BP_PickUp_Ring.BP_PickUp_Ring_C" (`KismetMathLibrary.MakeTransform` _end_location _returnvalue) "AdjustIfPossibleButAlwaysSpawn" "OverrideRootScale")))
    (:`==`
      (goto _label_4))
    (:`<`
      (`|SpawnActorFromClass` (select `bool` (`KismetMathLibrary.RandomBool`) :`false` "/Game/Blueprints/PickUp/BP_PickUpMushroom.BP_PickUpMushroom_C" :`true` "/Game/Blueprints/PickUp/BP_PickUp_Health.BP_PickUp_Health_C" :!type "/Game/Blueprints/PickUp/BP_PickUpBase Class Reference") (`KismetMathLibrary.MakeTransform` _end_location _returnvalue) "Undefined" "OverrideRootScale")))
  (`self.K2_DestroyActor`))

(fn `UserConstructionScript`
  (bind _returnvalue (`self.K2_GetActorLocation`))
  (`PaperFlipbookComponent.SetFlipbook` (`self.PaperFlipbook`) "/Game/Animations/Claw.Claw")
  (set `self.delta` 50.0)
  (`parent.UserConstructionScript`)
  (set `self.end_location` _returnvalue)
  (set `self.start_location` (`KismetMathLibrary.MakeVector` (.x _returnvalue) (.y _returnvalue) (- (.z _returnvalue) (* 3 (.z (`.BoxExtent` (`KismetSystemLibrary.GetComponentBounds` (`self.Box`)))))))))