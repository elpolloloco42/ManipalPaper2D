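; Hero "Braid" projectile built on a Paper sprite, which ignores its owner and expires after five seconds.
; On hitting anything else it disables collision and destroys itself after a short delay.
; Work is split by authority: the server damages AI enemies or other heroes, while remote instances hide the sprite and show an explosion particle.
; The construction script resets scale and clears the particle template on authority.
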(event `self.ReceiveBeginPlay`
  ;[1 0.121 0.2007] Begin Play / Destroy after 5sec
  (`|ExecutionSequence`
    (:`then_0`
      (`PrimitiveComponent.IgnoreActorWhenMoving` (`self.PaperSprite`) (`self.player_owner`) true))
    (:`then_1`
      (`KismetSystemLibrary.Delay` 5.0)
      (`self.K2_DestroyActor`))))

(event `self.ReceiveHit`
  (params (MyComp :type "PrimitiveComponent Object Reference") (Other :type "Actor Object Reference") (OtherComp :type "PrimitiveComponent Object Reference") (bSelfMoved :type Boolean) (HitLocation :type "Vector Structure") (HitNormal :type "Vector Structure") (NormalImpulse :type "Vector Structure") (Hit :type "HitResult Structure (by ref)"))
  ;[1 0.121 0.2007] Hit Event / Apply Damage On Server / Explose On Client
  (if (not (== Other (`self.player_owner`)))
    (`|ExecutionSequence`
      (:`then_0`
        (`PrimitiveComponent.SetCollisionResponseToAllChannels` (`self.PaperSprite`) "ECR_Ignore")
        (`KismetSystemLibrary.Delay` 3.0)
        (`self.K2_DestroyActor`))
      (:`then_1`
        (`/Engine/EditorBlueprintResources/ActorMacros.Switch Has Authority`
          (:`Authority`
            (bind _asbp_ia_enemie_base (cast `/Game/Blueprints/Characters/Enemies/BP_IA_Enemie_Base` Other)
              (:`then`
                (`GameplayStatics.ApplyDamage` _asbp_ia_enemie_base 1.0))
              (:`CastFailed`
                (bind _aspaper_2dhero_base (cast `/Game/Blueprints/Characters/Hero/Paper2DHeroBase` Other))
                (`GameplayStatics.ApplyDamage` _aspaper_2dhero_base 1.0 null self))))
          (:`Remote`
            (`SceneComponent.SetVisibility` (`self.PaperSprite`) false false)
            (`ParticleSystemComponent.SetTemplate` (`self.ParticleSystem`) "/Game/StarterContent/Particles/P_Explosion.P_Explosion")))))))

(fn `UserConstructionScript`
  (`self.SetActorScale3D` (1.0 1.0 1.0))
  (`/Engine/EditorBlueprintResources/ActorMacros.Switch Has Authority`
    (:`Authority`
      (`ParticleSystemComponent.SetTemplate` (`self.ParticleSystem`) null))))