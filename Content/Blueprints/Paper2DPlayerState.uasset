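; Player state for a 2D Paper2D hero, holding health, jump and dash limits, the current room and movement status flags.
; InitSpecs copies the limits from the hero and clears the dead and damaged flags, while ChangeRoom stores the room.
; AnimationStateMachine ranks flags by priority from death down to idle, returning the matching animation and whether it changed.
; Dash and climb reuse jump and run animations; attack has none assigned.
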(event `InitSpecs`
  (params (paper_player :type "/Game/Blueprints/Characters/Hero/Paper2DHero Object Reference"))
  ;[0.3059 1 0.2732] Set specs from hero
  (set `self.health` (`/Game/Blueprints/Characters/Hero/Paper2DHero.health` paper_player))
  (set `self.max_jump` (`/Game/Blueprints/Characters/Hero/Paper2DHero.max_jump` paper_player))
  (set `self.max_dash` (`/Game/Blueprints/Characters/Hero/Paper2DHero.max_dash` paper_player))
  (set `self.is_dead` false)
  (set `self.is_damaged` false))

(event `ChangeRoom`
  (params (room :type "/Game/Blueprints/Level/BP_Room Object Reference"))
  ;[0.3059 1 0.2732] Change Current Room
  (set `self.current_room` room))

(fn `AnimationStateMachine`
  (returns (changed :type Boolean) (animation :type "PaperFlipbook Object Reference"))
  (locals (animation_tmp :type "/Game/Data/E_AnimationState Enum"))
  (set `local.animation_tmp` (`self.animation`))
  (if (`self.is_dead`)
    (set `self.animation` "NewEnumerator9")
    (elif (`self.is_dashing`)
      (set `self.animation` "NewEnumerator3")
      (elif (`self.is_climbing`)
        (set `self.animation` "NewEnumerator7")
        (elif (`self.is_attacking`)
          (set `self.animation` "NewEnumerator4")
          (elif (`self.is_damaged`)
            (set `self.animation` "NewEnumerator8")
            (elif (`self.is_falling`)
              (set `self.animation` "NewEnumerator5")
              (elif (`self.is_start_falling`)
                (set `self.animation` "NewEnumerator6")
                (elif (`self.is_jumping`)
                  (set `self.animation` "NewEnumerator2")
                  (elif (`self.is_moving`)
                    (set `self.animation` "NewEnumerator1")
                    (else
                      (set `self.animation` "NewEnumerator0")))))))))))
  (return (`|EnumInequality` (`local.animation_tmp`) (`self.animation`)) (select `/Game/Data/E_AnimationState` (`self.animation`) :`NewEnumerator0` "/Game/Animations/hero_idle.hero_idle" :`NewEnumerator1` "/Game/Animations/hero_run.hero_run" :`NewEnumerator2` "/Game/Animations/jump_start.jump_start" :`NewEnumerator3` "/Game/Animations/jump_start.jump_start" :`NewEnumerator6` "/Game/Animations/jump_fall1.jump_fall1" :`NewEnumerator5` "/Game/Animations/jump_fall2.jump_fall2" :`NewEnumerator7` "/Game/Animations/hero_run.hero_run" :`NewEnumerator8` "/Game/Animations/hero_damage.hero_damage" :`NewEnumerator9` "/Game/Animations/death.death" :!type "PaperFlipbook Object Reference")))

(fn `UserConstructionScript`)